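; GA_FireSlash is a gameplay ability that casts the mage's fire slash attack.
; On activation it commits, casts the player character to BP_Mage and spawns a BP_FireSlash actor at the weapon's transform, handing it GE_ApplyDamage as its effect class.
; After a one-second delay it destroys the slash actor and ends the ability.
; A failed cast stops execution without ending the ability.
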(event `self.K2_ActivateAbility`
  (`self.K2_CommitAbility`)
  (bind _asbp_mage (cast `/Game/GameCore/Character/Characters/Mage/BP_Mage` (`GameplayStatics.GetPlayerCharacter` 0)))
  (bind _weapon (`/Game/GameCore/Character/Characters/BP_CustomHUD_Character.Weapon` _asbp_mage))
  (bind _returnvalue (`|SpawnActorFromClass` "/Game/BP_Actors/BP_FireSlash.BP_FireSlash_C" (`KismetMathLibrary.MakeTransform` (`SceneComponent.K2_GetComponentLocation` _weapon) (`SceneComponent.K2_GetComponentRotation` _weapon)) "Undefined" "OverrideRootScale" null "NewEnumerator0" "/Game/GAS/GameplayEffects/CharacterEffects/GE_ApplyDamage.GE_ApplyDamage_C" null))
  (`KismetSystemLibrary.Delay` 1.0)
  (`Actor.K2_DestroyActor` _returnvalue)
  (`self.K2_EndAbility`))