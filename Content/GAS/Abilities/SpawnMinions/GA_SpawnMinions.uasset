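; Gameplay ability that summons a group of BP_Minions around the player's mage.
; On activation it commits without branching on the result, then casts player 0's character to BP_Mage.
; A loop spawns each minion at a random reachable navigation point near the mage's mesh, matching the mesh rotation, then ends the ability.
; A failed cast stops execution before EndAbility is reached.
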(event `self.K2_ActivateAbility`
  (`self.K2_CommitAbility`)
  (bind _asbp_mage (cast `/Game/GameCore/Character/Characters/Mage/BP_Mage` (`GameplayStatics.GetPlayerCharacter` 0)))
  (for _ (range 4)
    (bind _mesh (`Character.Mesh` _asbp_mage))
    (`|SpawnActorFromClass` "/Game/GameCore/Character/Characters/Mage/BP_Minions.BP_Minions_C" (`KismetMathLibrary.MakeTransform` (`NavigationSystemV1.K2_GetRandomReachablePointInRadius` (`SceneComponent.K2_GetComponentLocation` _mesh) 400.0 null null) (`SceneComponent.K2_GetComponentRotation` _mesh)) "Undefined" "OverrideRootScale" null null))
  (`self.K2_EndAbility`))