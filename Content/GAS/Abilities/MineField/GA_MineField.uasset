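; Gameplay ability that gives the player's mage a temporary mine field.
; On activation it commits, casts player character 0 to BP_Mage, and spawns a BP_MineField scaled by MineFieldRadius.
; The field snaps to the mage's Arrow1 component, then is destroyed after a fixed delay as the ability ends.
; The commit result is unchecked, and a failed cast stops without ending the ability.
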(event `self.K2_ActivateAbility`
  (`self.K2_CommitAbility`)
  (bind _asbp_mage (cast `/Game/GameCore/Character/Characters/Mage/BP_Mage` (`GameplayStatics.GetPlayerCharacter` 0)))
  (bind _mesh (`Character.Mesh` _asbp_mage))
  (bind _returnvalue (`|SpawnActorFromClass` "/Game/BP_Actors/BP_MineField.BP_MineField_C" (`KismetMathLibrary.MakeTransform` (`SceneComponent.K2_GetComponentLocation` _mesh) (`SceneComponent.K2_GetComponentRotation` _mesh) (`self.MineFieldRadius`)) "Undefined" "OverrideRootScale" null _asbp_mage))
  (`Actor.K2_AttachToComponent` _returnvalue (`/Game/GameCore/Character/Characters/Mage/BP_Mage.Arrow1` _asbp_mage) "None" "SnapToTarget" "SnapToTarget" "KeepRelative" true)
  (`KismetSystemLibrary.Delay` 5.0)
  (`Actor.K2_DestroyActor` _returnvalue)
  (`self.K2_EndAbility`))