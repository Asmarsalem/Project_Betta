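; GA_Ricochet is a Gameplay Ability that fires a BP_EviliosArrow from the player's BP_Evilios character toward an AI.
; On activation it takes the first BP_AI found in the world, with no distance or targeting check, and aims from the ArrowOutput component at that actor's mesh.
; It spawns the arrow at double scale and ends immediately, so any ricochet behavior is not in this graph.
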(event `self.K2_ActivateAbility`
  (bind _asbp_evilios (cast `/Game/GameCore/Character/Characters/Evilios/BP_Evilios` (`GameplayStatics.GetPlayerCharacter` 0)))
  (bind _returnvalue (`GameplayStatics.GetActorOfClass` "/Game/Systems/WaveSystem/AI_system/AI/BP_AI.BP_AI_C"))
  (bind _returnvalue_2 (`SceneComponent.K2_GetComponentLocation` (`/Game/GameCore/Character/Characters/Evilios/BP_Evilios.ArrowOutput` _asbp_evilios)))
  (`|SpawnActorFromClass` "/Game/GameCore/Character/Characters/Evilios/BP_EviliosArrow.BP_EviliosArrow_C" (`KismetMathLibrary.MakeTransform` _returnvalue_2 (`KismetMathLibrary.FindLookAtRotation` _returnvalue_2 (`SceneComponent.K2_GetComponentLocation` (`Character.Mesh` _returnvalue))) (2.0 2.0 2.0)) "Undefined" "OverrideRootScale" null null)
  (`self.K2_EndAbility`))