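; GA_Poison is a gameplay ability that casts a poison spell on an enemy near the player.
; On activation it commits, then sphere-overlaps around the player's BP_CustomHUD_Character and tests only the first result for BPI_Enemy.
; A match spawns BP_PoisonSpell at that enemy's location with GE_Poison, an ice aura VFX and EarthquakeRadius as its radius.
; EndAbility runs only after that spawn, not when the cast or interface check fails.
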(event `self.K2_ActivateAbility`
  (`self.K2_CommitAbility`)
  (bind _asbp_custom_hud_character (cast `/Game/GameCore/Character/Characters/BP_CustomHUD_Character` (`GameplayStatics.GetPlayerCharacter` 0)))
  (bind _outactors (`KismetSystemLibrary.SphereOverlapActors` (`Actor.K2_GetActorLocation` _asbp_custom_hud_character) (`self.Sphere Radius`) (`|MakeArray` "ObjectTypeQuery9" :!type "EObjectTypeQuery Enum")))
  (bind _output (`|GetArrayItem` _outactors))
  (if (`KismetSystemLibrary.DoesImplementInterface` _output "/Game/Data/BP_Interface/BPI_Enemy.BPI_Enemy_C")
    (`|SpawnActorFromClass` "/Game/BP_Actors/BP_PoisonSpell.BP_PoisonSpell_C" (`KismetMathLibrary.Conv_VectorToTransform` (`Actor.K2_GetActorLocation` _output)) "Undefined" "OverrideRootScale" null (`self.Earthquake Radius`) "/Game/MapAssets/InfinityBladeEffects/Effects/FX_Skill_Aura/P_Aura_Ice_Upheaval_01.P_Aura_Ice_Upheaval_01" "/Game/GAS/GameplayEffects/CharacterEffects/GE_Poison.GE_Poison_C" null)
    (`self.K2_EndAbility`)))