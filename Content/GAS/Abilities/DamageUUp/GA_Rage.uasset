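; GA_Rage is a gameplay ability that puts the player's BP_Warzog character into a temporary rage state.
; On activation it prints a debug message, commits, enlarges the character mesh and applies the GE_Rage effect through the ability system component.
; After a fixed delay it sets the mesh scale to unit size, rather than the stored original, and ends the ability without explicitly removing the effect.
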(event `self.K2_ActivateAbility`
  (`KismetSystemLibrary.PrintString` "Raged" true true (struct :`R` 1.0 :`G` 0.152418 :`B` 0.102654 :`A` 1.0))
  (`self.K2_CommitAbility`)
  (bind _asbp_warzog (cast `/Game/Demo/Examples/CustomHUD/Characters/Warzog/BP_Warzog` (`GameplayStatics.GetPlayerCharacter` 0)))
  (bind _mesh (`Character.Mesh` _asbp_warzog))
  (`SceneComponent.SetWorldScale3D` _mesh (+ (`SceneComponent.K2_GetComponentScale` _mesh) (0.5 0.5 0.5)))
  (`AbilitySystemComponent.BP_ApplyGameplayEffectToSelf` :`self` (`AbilitySystemBlueprintLibrary.GetAbilitySystemComponent` _asbp_warzog) :`GameplayEffectClass` "/Game/Demo/Examples/CustomHUD/AbilitySystem/GameplayEffects/CharacterEffects/GE_Rage.GE_Rage_C")
  (`KismetSystemLibrary.Delay` 6.0)
  (`SceneComponent.SetWorldScale3D` _mesh (1.0 1.0 1.0))
  (`self.K2_EndAbility`))