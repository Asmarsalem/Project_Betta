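; GA_Lightning is a gameplay ability that strikes a nearby enemy with lightning.
; It commits, prints a debug value and runs a sphere overlap around the player character, sized by a float attribute of the owning actor.
; If the first overlapped actor implements BPI_Enemy, it spawns BP_Lightning there, passing radius, VFX and GE_Lightning effect.
; The ability ends only on that successful branch.
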(event `self.K2_ActivateAbility`
  (bind (_bsuccessfullyfoundattribute _returnvalue) (`AbilitySystemBlueprintLibrary.GetFloatAttribute` (`self.GetOwningActorFromActorInfo`) (struct :`AttributeName` "lighting" :`Attribute` "/Script/GASCompanionDemo.XPAttributeSet:lighting" :`AttributeOwner` "/Script/CoreUObject.Class'\"/Script/GASCompanionDemo.XPAttributeSet\"'")))
  (`self.K2_CommitAbility`)
  (bind _asbp_custom_hud_character (cast `/Game/GameCore/Character/Characters/BP_CustomHUD_Character` (`GameplayStatics.GetPlayerCharacter` 0)))
  (`KismetSystemLibrary.PrintString` (`KismetStringLibrary.Conv_DoubleToString` _returnvalue) true true (struct :`R` 1.0 :`G` 0.329115 :`B` 0.617252 :`A` 1.0))
  (bind _outactors (`KismetSystemLibrary.SphereOverlapActors` (`Actor.K2_GetActorLocation` _asbp_custom_hud_character) _returnvalue (`|MakeArray` "ObjectTypeQuery9" :!type "EObjectTypeQuery Enum")))
  (bind _output (`|GetArrayItem` _outactors))
  (if (`KismetSystemLibrary.DoesImplementInterface` _output "/Game/Data/BP_Interface/BPI_Enemy.BPI_Enemy_C")
    (`|SpawnActorFromClass` "/Game/BP_Actors/BP_Lightning.BP_Lightning_C" (`KismetMathLibrary.Conv_VectorToTransform` (`Actor.K2_GetActorLocation` _output)) "Undefined" "OverrideRootScale" null (`self.Lightning Radius`) "/Game/MapAssets/InfinityBladeEffects/Effects/FX_Mobile/Lightning/P_LineToPoint_Blast_Lightning_00.P_LineToPoint_Blast_Lightning_00" "/Game/GAS/GameplayEffects/CharacterEffects/GE_Lightning.GE_Lightning_C" null)
    (`self.K2_EndAbility`)))