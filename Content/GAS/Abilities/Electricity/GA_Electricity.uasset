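; Gameplay ability that strikes actors around the player with electricity.
; On activation it commits, then runs a sphere overlap at the player character's Box component, filtered to one object type.
; Each actor found gets a BP_Electricity spawned and attached to it, configured with the GE_Lightning effect and an ice aura circle particle as damage VFX.
; The ability ends immediately after spawning, leaving any further behavior to those spawned actors.
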(event `self.K2_ActivateAbility`
  (`self.K2_CommitAbility`)
  (bind _asbp_custom_hud_character (cast `/Game/Demo/Examples/CustomHUD/BP_CustomHUD_Character` (`GameplayStatics.GetPlayerCharacter` 0)))
  (bind _outactors (`KismetSystemLibrary.SphereOverlapActors` (`SceneComponent.K2_GetComponentLocation` (`/Game/Demo/Examples/CustomHUD/BP_CustomHUD_Character.Box` _asbp_custom_hud_character)) (`self.Sphere Radius`) (`|MakeArray` "ObjectTypeQuery9" :!type "EObjectTypeQuery Enum")))
  (for _array_element _outactors
    (bind _returnvalue (`|SpawnActorFromClass` "/Game/BP_Actors/BP_Electricity.BP_Electricity_C" (`Actor.GetTransform` _array_element) "Undefined" "OverrideRootScale" null 100.0 "/Game/InfinityBladeEffects/Effects/FX_Mobile/ICE/combat/P_AuraCircle_Ice_00.P_AuraCircle_Ice_00" "/Game/GAS/GameplayEffects/CharacterEffects/GE_Lightning.GE_Lightning_C" null))
    (`Actor.K2_AttachToActor` _returnvalue _array_element "None" "SnapToTarget" "KeepRelative" "KeepRelative" true))
  (`self.K2_EndAbility`))