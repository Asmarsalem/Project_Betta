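; BP_EXP is an experience pickup actor that grants XP when collected.
; EV_AttachToActor plays the Attach timeline to pull the pickup toward the given actor in X and Y, keeping its own height and re-reading both locations each update.
; EV_CollectEnergy destroys the pickup, then on authority calls ADDXP on BP_CustomHUD_GameMode.
; Both events are triggered from outside, as BeginPlay and overlap are unused.
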(event `EV_CollectEnergy`
  (`self.K2_DestroyActor`)
  (`/Engine/EditorBlueprintResources/ActorMacros.Switch Has Authority`
    (:`Authority`
      (bind _asbp_custom_hud_game_mode (cast `/Game/GameCore/GameMode/BP_CustomHUD_GameMode` (`GameplayStatics.GetGameMode`)))
      (`/Game/GameCore/GameMode/BP_CustomHUD_GameMode.ADDXP` _asbp_custom_hud_game_mode))))

(event `EV_AttachToActor`
  (params (NewParam :type "Actor Object Reference"))
  (bind (_returnvalue_x _returnvalue_y _returnvalue_z) (`KismetMathLibrary.BreakVector` (`self.K2_GetActorLocation`)))
  (bind (_returnvalue_x_2 _returnvalue_y_2) (`KismetMathLibrary.BreakVector` (`self.K2_GetActorLocation` NewParam)))
  (bind (_direction _floattrack) (`Timeline|Attach`)
    (:`Update`
      (`self.K2_SetActorLocation` (`KismetMathLibrary.VLerp` (`KismetMathLibrary.MakeVector` _returnvalue_x _returnvalue_y _returnvalue_z) (`KismetMathLibrary.MakeVector` _returnvalue_x_2 _returnvalue_y_2 _returnvalue_z) _floattrack)))))

(fn `UserConstructionScript`)