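; Boss enemy Blueprint that provides the boss's projectile and lightning attacks as callable events.
; Single shots are time-throttled, while the three-arrow spread and the radial Ultimate use DoOnce gates reset by timers.
; The Ultimate also calls a dispatcher with its cooldown time.
; Lightning spawns BP_BossLightning markers around and on the player, then after a delay replaces all with BP_BossBaseAbility actors carrying the lightning effect and VFX.
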(event `self.ReceiveBeginPlay`
  ;[1 1 1] Begin
  (`parent.ReceiveBeginPlay`))

(event `Lightning_Circle`
  (bind _mesh (`Character.Mesh` (`GameplayStatics.GetPlayerCharacter` 0)))
  (bind (_returnvalue_x _returnvalue_y _returnvalue_z) (`KismetMathLibrary.BreakVector` (`SceneComponent.K2_GetComponentLocation` _mesh)))
  ;[0 1 0.1529] Lightining Function
  (`KismetSystemLibrary.PrintString` "activated")
  (for _index (range 1 6)
    (bind _output_get (set `self.Angle` (* (/ (`self.360`) (`self.NbOfCircles`)) _index)))
    (set `self.AngleRad` (`KismetMathLibrary.DegreesToRadians` _output_get))
    (`|SpawnActorFromClass` "/Game/BP_Actors/BP_BossLightning.BP_BossLightning_C" (`KismetMathLibrary.MakeTransform` (`KismetMathLibrary.MakeVector` (* (+ _returnvalue_x (`self.CircleRadius`)) (`KismetMathLibrary.Cos` (`self.AngleRad`))) (* (+ _returnvalue_y (`self.CircleRadius`)) (`KismetMathLibrary.Sin` (`self.AngleRad`))) _returnvalue_z) (`SceneComponent.K2_GetComponentRotation` _mesh)) "Undefined" "OverrideRootScale" null null))
  (`self.ApplyLightning`))

(event `ApplyLightning`
  ;[0 1 0.1529] Apply VFX
  (`|SpawnActorFromClass` "/Game/BP_Actors/BP_BossLightning.BP_BossLightning_C" (`KismetMathLibrary.Conv_VectorToTransform` (`SceneComponent.K2_GetComponentLocation` (`Character.Mesh` (`GameplayStatics.GetPlayerCharacter` 0)))) "Undefined" "OverrideRootScale" null null)
  (`KismetSystemLibrary.Delay` (`self.DelayOfLightning`))
  (bind _outactors (`GameplayStatics.GetAllActorsOfClass` "/Game/BP_Actors/BP_BossLightning.BP_BossLightning_C"))
  (for _array_element _outactors
    (`|SpawnActorFromClass` "/Game/BP_Actors/BP_BossBaseAbility.BP_BossBaseAbility_C" (`KismetMathLibrary.Conv_VectorToTransform` (`self.K2_GetActorLocation` _array_element)) "Undefined" "OverrideRootScale" null 50.0 "/Game/GAS/GameplayEffects/GE_BossLightning.GE_BossLightning_C" "/Game/MapAssets/InfinityBladeEffects/Effects/FX_Mobile/Lightning/P_LineToPoint_Blast_Lightning_00.P_LineToPoint_Blast_Lightning_00" null)
    (`self.K2_DestroyActor` _array_element)))

(event `attack_multiple_bullets`
  (bind _returnvalue (`SceneComponent.K2_GetComponentRotation` (`self.StaticMesh`)))
  ;[0 1 0.1529] 3 bullets Attack
  (`/Engine/EditorBlueprintResources/StandardMacros.DoOnce` false :!label _label
    (:`Completed`
      (for _index (range -1 2)
        (`|SpawnActorFromClass` "/Game/BP_Actors/BP_AIArrow.BP_AIArrow_C" (`KismetMathLibrary.MakeTransform` (+ (`SceneComponent.K2_GetComponentLocation` (`self.StaticMesh`)) (`KismetMathLibrary.GreaterGreater_VectorRotator` (-40.0 0.0 0.0) _returnvalue)) (`KismetMathLibrary.MakeRotator` 0.0 0.0 (+ (* _index 15) (.yaw _returnvalue)))) "Undefined" "OverrideRootScale" null null)
        (bind _returnvalue_2 (`KismetSystemLibrary.K2_SetTimerDelegate` (delegate `Cooldown3bulletts`) (`self.Time_3bullets`)))))))

(event `ShootBoss`
  (bind _returnvalue (`KismetSystemLibrary.GetGameTimeInSeconds`))
  (bind _returnvalue_2 (`self.K2_GetActorRotation`))
  (bind _xshoot (`self.XShoot`))
  ;[0 1 0.1529] Boss_Shooting
  (if (== _xshoot 0.0)
    (set `self.XShoot` _returnvalue :!label _label_2)
    (`|SpawnActorFromClass` "/Game/BP_Actors/BP_AIArrow.BP_AIArrow_C" (`KismetMathLibrary.MakeTransform` (+ (`SceneComponent.K2_GetComponentLocation` (`self.StaticMesh`)) (`KismetMathLibrary.GreaterGreater_VectorRotator` (-40.0 0.0 0.0) _returnvalue_2)) _returnvalue_2) "Undefined" "OverrideRootScale" null null)
    (elif (not (> (+ _xshoot 0.9) _returnvalue))
      (goto _label_2))))

(event `Cooldown3bulletts`
  ;[0 1 0.1529] 3 bullets Attack
  (`KismetSystemLibrary.K2_ClearAndInvalidateTimerHandle` (stale `attack_multiple_bullets` _returnvalue_2))
  (goto _label :!via `Reset`))

(event `360Shoot`
  ;[0 0 0] Ult Damage
  (`/Engine/EditorBlueprintResources/StandardMacros.DoOnce` false :!label _label_3
    (:`Completed`
      (`self.Ultimate`)
      (bind _returnvalue (`KismetSystemLibrary.K2_SetTimerDelegate` (delegate `Cooldown`) (`self.Time_ult`))))))

(event `Cooldown`
  ;[0 0 0] Ult Damage
  (`KismetSystemLibrary.K2_ClearAndInvalidateTimerHandle` (stale `360Shoot` _returnvalue))
  (goto _label_3 :!via `Reset`))

(event `StopShoot`
  ;[0 0 0] Ult Damage
  ;;[1 0.0101 0] Active Event
)

(fn `Ultimate`
  (for _index (range -18 19)
    (`|SpawnActorFromClass` "/Game/BP_Actors/BP_AIArrow.BP_AIArrow_C" (`KismetMathLibrary.MakeTransform` (+ (`SceneComponent.K2_GetComponentLocation` (`self.StaticMesh`)) (`KismetMathLibrary.GreaterGreater_VectorRotator` (-40.0 0.0 0.0) (`self.K2_GetActorRotation`))) (`KismetMathLibrary.MakeRotator` 0.0 0.0 (`KismetMathLibrary.Conv_IntToDouble` (* _index 20)))) "Undefined" "OverrideRootScale" null null)
    (`self.Ult_Dispatcher` (`self.Time_ult`))))

(fn `UserConstructionScript`
  (`parent.UserConstructionScript`))