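; BP_RangedAI is a ranged child AI in the wave system that fires arrows at players in front of it.
; BeginPlay sets the attack range, and Tick derives its own interval from an ability system float attribute, so each tick is one attack attempt.
; Each attempt line-traces forward from an arrow component and spawns BP_AIArrow when the hit actor implements BPI_Player.
; Debug trace drawing and result printing are left on.
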(event `self.ReceiveBeginPlay`
  (`parent.ReceiveBeginPlay`)
  (set `self.AI Range Attack` (`self.RangedAI_AttackRange`)))

(event `self.ReceiveTick`
  (params (DeltaSeconds :type "Float (single-precision)"))
  (bind _output_get (set `self.AI Attack Speed` (/ (`.ReturnValue` (`AbilitySystemBlueprintLibrary.GetFloatAttributeFromAbilitySystemComponent` (`self.GSCAbilitySystem`) (struct :`AttributeName` "AttackSpeed" :`Attribute` "/Script/GASCompanionDemo.MainAttributes:AttackSpeed" :`AttributeOwner` "/Script/CoreUObject.Class'\"/Script/GASCompanionDemo.MainAttributes\"'"))) -10.0)))
  (`self.SetActorTickInterval` _output_get)
  (`self.Ranged AutoAttack`))

(fn `Ranged AutoAttack`
  (bind _arrow1 (`self.Arrow1`))
  (bind _arrow1_2 (`self.Arrow1`))
  (bind _returnvalue (`SceneComponent.K2_GetComponentLocation` _arrow1_2))
  (bind _outhit (`KismetSystemLibrary.LineTraceSingle` :`Start` _returnvalue :`End` (+ _returnvalue (* (`SceneComponent.GetForwardVector` _arrow1_2) 1000.0)) :`TraceChannel` "TraceTypeQuery2" :`DrawDebugType` "ForDuration"))
  (bind _returnvalue_2 (`KismetSystemLibrary.DoesImplementInterface` (`.HitActor` (`GameplayStatics.BreakHitResult` _outhit)) "/Game/Data/BP_Interface/BPI_Player.BPI_Player_C"))
  (if _returnvalue_2
    (`|SpawnActorFromClass` "/Game/BP_Actors/BP_AIArrow.BP_AIArrow_C" (`KismetMathLibrary.MakeTransform` (`SceneComponent.K2_GetComponentLocation` _arrow1) (`KismetMathLibrary.Conv_VectorToRotator` (`SceneComponent.GetForwardVector` _arrow1)) (2.0 2.0 2.0)) "Undefined" "OverrideRootScale" null null)
    (`KismetSystemLibrary.PrintString` (`KismetStringLibrary.Conv_BoolToString` _returnvalue_2))
    (else
      (`KismetSystemLibrary.PrintString` (`KismetStringLibrary.Conv_BoolToString` _returnvalue_2)))))

(fn `UserConstructionScript`
  (`parent.UserConstructionScript`))