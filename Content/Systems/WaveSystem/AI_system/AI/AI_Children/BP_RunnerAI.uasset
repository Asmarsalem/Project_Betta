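; BP_RunnerAI is a child AI character in the wave system that periodically changes its movement speed in bursts.
; After the parent BeginPlay, a looping 12-second timer sets max walk speed to the Acceleration variable for four seconds.
; It then resets the speed from a float attribute on the GSC ability system component, printing the speed after each change.
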(event `self.ReceiveBeginPlay`
  (`parent.ReceiveBeginPlay`)
  (`KismetSystemLibrary.K2_SetTimerDelegate` (delegate `AI_Acceleration`) 12.0 true))

(event `AI_Acceleration`
  ;[0.07227 0.2462 0.0382] Acceleration
  (bind _output_get (set `CharacterMovementComponent.MaxWalkSpeed` (`self.Acceleration `) (`self.CharacterMovement`)))
  (`KismetSystemLibrary.PrintString` (`KismetStringLibrary.Conv_DoubleToString` _output_get))
  (`KismetSystemLibrary.Delay` 4.0)
  (bind _output_get_2 (set `CharacterMovementComponent.MaxWalkSpeed` (`.ReturnValue` (`AbilitySystemBlueprintLibrary.GetFloatAttributeFromAbilitySystemComponent` (`self.GSCAbilitySystem`) (struct :`AttributeName` "Speed" :`Attribute` "/Script/GASCompanionDemo.MainAttributes:Speed" :`AttributeOwner` "/Script/CoreUObject.Class'\"/Script/GASCompanionDemo.MainAttributes\"'"))) (`self.CharacterMovement`)))
  (`KismetSystemLibrary.PrintString` (`KismetStringLibrary.Conv_DoubleToString` _output_get_2)))

(fn `UserConstructionScript`
  (`parent.UserConstructionScript`))