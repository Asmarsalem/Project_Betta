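; AI controller for ranged enemies that runs the BT_Ranged behavior tree and keeps focus on the player.
; On BeginPlay it starts the tree and caches its pawn and the player.
; Sight updates from AI perception set the TargetActor blackboard key to the player, or clear it and store LastKnownLocation when sight is lost.
; Tick sets focus on the player's BP_Anubis character every frame, independent of perception.
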(event `self.ReceiveBeginPlay`
  (`self.RunBehaviorTree` "/Game/Systems/WaveSystem/AI_system/AI/AI_Children/Ai_Ranged/BT_Ranged.BT_Ranged")
  (bind _asbp_ai (cast `/Game/Systems/WaveSystem/AI_system/AI/BP_AI` (`self.K2_GetPawn`)))
  (set `self.As BP AI` _asbp_ai)
  (set `self.targetlocation` (`GameplayStatics.GetPlayerCharacter` 0)))

(event `self.ReceiveTick`
  (params (DeltaSeconds :type "Float (single-precision)"))
  (bind _asbp_anubis (cast `/Game/GameCore/Character/Characters/Anubis/BP_Anubis` (`GameplayStatics.GetPlayerCharacter` 0)))
  (`self.K2_SetFocus` self _asbp_anubis))

(event `self.AIPerception.OnTargetPerceptionUpdated`
  (params (Actor :type "Actor Object Reference") (Stimulus :type "AIStimulus Structure"))
  (`self.HandleSightSense` Actor Stimulus))

(fn `HandleSightSense`
  (params (Actor :type "Actor Object Reference") (Stimlus :type "AIStimulus Structure"))
  (bind (_stimlus_age _stimlus_expirationage _stimlus_strength _stimlus_stimuluslocation _stimlus_receiverlocation _stimlus_tag _stimlus_bsuccessfullysensed) (break `AIStimulus` (`local.Stimlus`)))
  (bind _returnvalue (`AIPerceptionSystem.GetSenseClassForStimulus` Stimlus))
  (if (== _returnvalue "/Script/AIModule.AISense_Sight")
    (if (== (`local.Actor`) (`GameplayStatics.GetPlayerCharacter` 0))
      (`BlackboardComponent.SetValueAsObject` (`self.Blackboard`) "TargetActor" (`KismetMathLibrary.SelectObject` (`GameplayStatics.GetPlayerCharacter` 0) null _stimlus_bsuccessfullysensed))
      (if (not _stimlus_bsuccessfullysensed)
        (`BlackboardComponent.SetValueAsVector` (`self.Blackboard`) "LastKnownLocation" _stimlus_stimuluslocation))
      (else
        (return)))
    (else
      (return))))

(fn `UserConstructionScript`)