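; Ranged enemy AI pawn in the wave system that chases player 0 and fires arrows once in range.
; Tick re-issues AIMoveTo toward the player; success calls Shoot, while failure calls an empty StopShoot.
; Shoot spawns BP_AIArrow from the Arrow1 component, rate-limited by a game-time stamp in XShoot.
; RangedAutoAttack, uncalled here, is a line-trace variant that fires only on BPI_Player hits and prints debug output.
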(event `self.ReceiveTick`
  (params (DeltaSeconds :type "Float (single-precision)"))
  (`|AIMoveTo` self (0.0 0.0 0.0) (`GameplayStatics.GetPlayerCharacter` 0) 450.0
    (:`OnSuccess`
      (`self.Shoot`))
    (:`OnFail`
      (`self.StopShoot`))))

(event `StopShoot`
  ;[0 1 0.1005] Shooting system
  ;;[0.9948 0.1068 0] Dont Delete This is an Active Event
)

(event `Shoot`
  (bind _returnvalue (`KismetSystemLibrary.GetGameTimeInSeconds`))
  (bind _returnvalue_2 (`self.K2_GetActorRotation`))
  (bind _xshoot (`self.XShoot`))
  ;[0 1 0.1005] Shooting system
  (if (== _xshoot 0.0)
    (set `self.XShoot` _returnvalue :!label _label)
    (`|SpawnActorFromClass` "/Game/BP_Actors/BP_AIArrow.BP_AIArrow_C" (`KismetMathLibrary.MakeTransform` (+ (`SceneComponent.K2_GetComponentLocation` (`self.Arrow1`)) (`KismetMathLibrary.GreaterGreater_VectorRotator` (-40.0 0.0 0.0) _returnvalue_2)) _returnvalue_2 (2.0 2.0 2.0)) "Undefined" "OverrideRootScale" null null)
    (elif (not (> (+ _xshoot 0.9) _returnvalue))
      (goto _label))))

(fn `Ranged AutoAttack`
  (bind _arrow1 (`self.Arrow1`))
  (bind _arrow1_2 (`self.Arrow1`))
  (bind _returnvalue (`SceneComponent.K2_GetComponentLocation` _arrow1_2))
  (bind _outhit (`KismetSystemLibrary.LineTraceSingle` :`Start` _returnvalue :`End` (+ _returnvalue (* (`SceneComponent.GetForwardVector` _arrow1_2) 1000.0)) :`TraceChannel` "TraceTypeQuery2" :`DrawDebugType` "ForDuration"))
  (bind _returnvalue_2 (`KismetSystemLibrary.DoesImplementInterface` (`.HitActor` (`GameplayStatics.BreakHitResult` _outhit)) "/Game/Data/BP_Interface/BPI_Player.BPI_Player_C"))
  (if _returnvalue_2
    (`|SpawnActorFromClass` "/Game/BP_Actors/BP_AIArrow.BP_AIArrow_C" (`KismetMathLibrary.MakeTransform` (`SceneComponent.K2_GetComponentLocation` _arrow1) (`KismetMathLibrary.Conv_VectorToRotator` (`SceneComponent.GetForwardVector` _arrow1)) (2.0 2.0 2.0)) "Undefined" "OverrideRootScale" null null)
    (`KismetSystemLibrary.PrintString` (`KismetStringLibrary.Conv_BoolToString` _returnvalue_2))
    (else
      (`KismetSystemLibrary.PrintString` (`KismetStringLibrary.Conv_BoolToString` _returnvalue_2)))))

(fn `UserConstructionScript`
  (`parent.UserConstructionScript`))