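; Boss AI character Blueprint with an unfinished ranged attack.
; RangedAttack calls PlayAnimMontage and stores the returned length in RangedAttackLength.
; FireProjectile_boss is an empty event; a disconnected SpawnActor node and an unused look-at rotation from FirePointBoss toward the player remain in the graph.
; BeginPlay, overlap and Tick are disabled, and construction only calls the parent.
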(event `Ranged Attack`
  (bind _returnvalue (`self.PlayAnimMontage` null))
  (set `self.RangedAttackLength` _returnvalue))

(event `FireProjectile_boss`)

(fn `UserConstructionScript`
  (`parent.UserConstructionScript`))