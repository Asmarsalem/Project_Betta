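; Boss AI Blueprint whose only active logic is the Lightning_Circle event, an attack meant to ring the player character with lightning.
; The event loops five times, spawning BP_BossLightning at angles stepped by NbOfCircles, using the player mesh's height and rotation.
; CircleRadius is added to player X/Y before the cos/sin multiply, so the ring centres on world origin rather than the player.
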(event `Lightning_Circle`
  (`KismetSystemLibrary.PrintString` "activated")
  (bind _asbp_custom_hud_character (cast `/Game/GameCore/Character/Characters/BP_CustomHUD_Character` (`GameplayStatics.GetPlayerCharacter` 0)))
  (for _index (range 1 6)
    (bind _output_get (set `self.Angle` (* (/ (`self.360`) (`self.NbOfCircles`)) _index)))
    (set `self.AngleRad` (`KismetMathLibrary.DegreesToRadians` _output_get))
    (bind _mesh (`Character.Mesh` _asbp_custom_hud_character))
    (bind (_returnvalue_x _returnvalue_y _returnvalue_z) (`KismetMathLibrary.BreakVector` (`SceneComponent.K2_GetComponentLocation` _mesh)))
    (`|SpawnActorFromClass` "/Game/BP_Actors/BP_BossLightning.BP_BossLightning_C" (`KismetMathLibrary.MakeTransform` (`KismetMathLibrary.MakeVector` (* (+ _returnvalue_x (`self.CircleRadius`)) (`KismetMathLibrary.Cos` (`self.AngleRad`))) (* (+ _returnvalue_y (`self.CircleRadius`)) (`KismetMathLibrary.Sin` (`self.AngleRad`))) _returnvalue_z) (`SceneComponent.K2_GetComponentRotation` _mesh)) "Undefined" "OverrideRootScale" null null))
  (`KismetSystemLibrary.PrintString` "Done"))

(event `self.ReceiveBeginPlay`)

(fn `UserConstructionScript`
  (`parent.UserConstructionScript`))