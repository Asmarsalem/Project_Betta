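; AI character Blueprint with an overhead-style status widget for health, built on GSCCoreComponent and the Gameplay Ability System.
; Health changes refresh the bar through a multicast and show the widget for a few seconds on a timer.
; Death stops AI logic, then multicasts ragdoll and widget hiding.
; Lethal damage grants the source character XP via a SetByCaller gameplay effect, and landing sends a gameplay event for the jump ability.
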(event `self.ReceiveBeginPlay`
  ;[0 0 0 0] Update Health Bar on Begin Play
  (`self.Multicast_UpdateHealthBar`))

(event `ShowStatusBarForDuration`
  (params (Duration :type "Float (double-precision)"))
  ;[0 0 0] Show Status Bar Widget for a given duration
  (`KismetSystemLibrary.K2_ClearAndInvalidateTimerHandle` (`self.ShowStatusBarTimer`))
  (if (`GSCCoreComponent.IsAlive` (`self.GSCCoreComponent`))
    (`SceneComponent.SetHiddenInGame` (`self.StatusWidgetComponent`) false false)
    (bind _returnvalue (`KismetSystemLibrary.K2_SetTimerDelegate` (delegate `HideWidgetTimer`) Duration))
    (set `self.ShowStatusBarTimer` _returnvalue)))

(event `HideWidgetTimer`
  ;[0 0 0] Show Status Bar Widget for a given duration
  (`KismetSystemLibrary.K2_ClearAndInvalidateTimerHandle` (`self.ShowStatusBarTimer`))
  (`self.HideStatusWidget`))

(event `self.OnLanded`
  (params (Hit :type "HitResult Structure (by ref)"))
  ;[0 0 0] Jump Ability needs to know when it ends
  (`AbilitySystemBlueprintLibrary.SendGameplayEventToActor` self))

(event `self.GSCCoreComponent.OnHealthChange`
  (params (DeltaValue :type "Float (single-precision)") (EventTags :type "GameplayTagContainer Structure"))
  ;[0 0 0] Update Status Widget bar on health change
  (`self.Multicast_UpdateHealthBar`)
  (`self.ShowStatusBarForDuration` 3.0))

(event `self.GSCCoreComponent.OnDeath`
  ;[0 0 0] OnDeath: Stop AI Logic, Activate Ragdoll, Hide Status Widget
  (bind _asbp_aicontroller (cast `/Game/Demo/Examples/Playground/AI/BP_AIController` (`self.GetController`)))
  (`BrainComponent.StopLogic` (`AIController.BrainComponent` _asbp_aicontroller) "You dead")
  (`self.Multicast_Ragdoll` true)
  (`self.Multicast_HideStatusWidget`))

(event `Multicast_UpdateHealthBar`
  (bind _gsccorecomponent (`self.GSCCoreComponent`))
  ;[0 0 0] Update Health Bar (Multicast)
  (`KismetSystemLibrary.Delay` 0.1)
  (if (!= (`GSCCoreComponent.GetMaxHealth` (`self.GSCCoreComponent`)) 0.0)
    (`/Engine/EditorBlueprintResources/StandardMacros.IsValid` (`self.StatusBarWidget`)
      (:`Is Valid`
        _)
      (:`Is Not Valid`
        (bind _aswb_status_bar (cast `/Game/Demo/Examples/Playground/UI/WB_StatusBar` (`WidgetComponent.GetUserWidgetObject` (`self.StatusWidgetComponent`))))
        (set `self.StatusBarWidget` _aswb_status_bar)))
    (`ProgressBar.SetPercent` (`/Game/Demo/Examples/Playground/UI/WB_StatusBar.HealthProgressBar` (`self.StatusBarWidget`)) (/ (`GSCCoreComponent.GetHealth` _gsccorecomponent) (`GSCCoreComponent.GetMaxHealth` _gsccorecomponent)))))

(event `Multicast_Ragdoll`
  (params (bNewSimulate :type Boolean))
  ;[0 0 0] Ragdoll (Multicast)
  (`SkeletalMeshComponent.SetAllBodiesSimulatePhysics` (`self.Mesh`) bNewSimulate)
  (`PrimitiveComponent.SetSimulatePhysics` (`self.Mesh`) bNewSimulate)
  (`PrimitiveComponent.WakeAllRigidBodies` (`self.Mesh`)))

(event `HideStatusWidget`
  ;[0 0 0] HideStatusWidget
  (`SceneComponent.SetHiddenInGame` (`self.StatusWidgetComponent`) true false))

(event `Multicast_HideStatusWidget`
  ;[0 0 0] HideStatusWidget
  (`self.HideStatusWidget`))

(event `Server_HideStatusWidget`
  ;[0 0 0] HideStatusWidget
  (`self.HideStatusWidget`))

(event `OwningClient_HideStatusWidget`
  ;[0 0 0] HideStatusWidget
  (`self.HideStatusWidget`))

(event `self.ReceiveTick`
  (params (DeltaSeconds :type "Float (single-precision)"))
  ;[0 0 0] Test
)

(event `self.GSCCoreComponent.OnDamage`
  (params (DamageAmount :type "Float (single-precision)") (SourceCharacter :type "Actor Object Reference") (DamageTags :type "GameplayTagContainer Structure (by ref)"))
  (bind _returnvalue (`AbilitySystemBlueprintLibrary.GetAbilitySystemComponent` SourceCharacter))
  (if (not (`GSCCoreComponent.IsAlive` (`self.GSCCoreComponent`)))
    ;[0 0 0] TODO: Should probably passed in OnDeath information about damage causer
    (bind _returnvalue_2 (`AbilitySystemBlueprintLibrary.AssignTagSetByCallerMagnitude` (`AbilitySystemComponent.MakeOutgoingSpec` :`self` _returnvalue :`GameplayEffectClass` "/Game/GAS/GameplayEffects/GE_XP_Add.GE_XP_Add_C") (struct :`TagName` "GameplayEffect.XP.Magnitude") (`self.GrantedXP`)))
    (`AbilitySystemComponent.BP_ApplyGameplayEffectSpecToSelf` _returnvalue _returnvalue_2)))

(fn `UserConstructionScript`)