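; Melee enemy AI for the wave system, using the Gameplay Ability System through GSC components.
; Pawn sensing moves it to player 0 and plays an attack montage at an attribute-driven rate; sphere overlaps during attacks apply a damage effect.
; Zero health destroys it, and EndPlay on authority updates the game mode's per-kill damage bonus and spawns EXP and random loot.
; A separate line-trace melee function is defined but not called here.
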(event `self.ReceiveBeginPlay`
  ;[0.00947 0 1] Begin
  (`GameplayStatics.SpawnEmitterAtLocation` "/Game/MapAssets/InfinityBladeEffects/Effects/FX_Mobile/ICE/combat/P_YoYo_IceBlast_Axe_00.P_YoYo_IceBlast_Axe_00" (`self.K2_GetActorLocation` self)))

(event `Get Number of Starting AI`
  ;[0.2257 1 0.7464] Set Number of Starting AI
  (bind _outactors (`GameplayStatics.GetAllActorsOfClass` "BP_AI_C"))
  (set `self.NumberOfDeployedAI` (`KismetArrayLibrary.Array_Length` _outactors)))

(event `Set AI Attack Speed`
  ;[0.03212 1 0] Set AI Attack Speed
  (set `self.AI Attack Speed` (/ (`.ReturnValue` (`AbilitySystemBlueprintLibrary.GetFloatAttributeFromAbilitySystemComponent` (`self.GSCAbilitySystem`) (struct :`AttributeName` "AttackSpeed" :`Attribute` "/Script/GASCompanionDemo.MainAttributes:AttackSpeed" :`AttributeOwner` "/Script/CoreUObject.Class'\"/Script/GASCompanionDemo.MainAttributes\"'"))) -10.0)))

(event `self.ReceiveEndPlay`
  (params (EndPlayReason :type "EEndPlayReason Enum" :default "Destroyed"))
  ;[0.6937 1 0.447] AI Death
  (`/Engine/EditorBlueprintResources/ActorMacros.Switch Has Authority`
    (:`Authority`
      (`|ExecutionSequence`
        (:`then_0`
          (bind _asbp_custom_hud_game_mode (cast `/Game/GameCore/GameMode/BP_CustomHUD_GameMode` (`GameplayStatics.GetGameMode`)))
          (bind _output_get (set `/Game/GameCore/GameMode/BP_CustomHUD_GameMode.IncreaseDamagePerKill` 0 _asbp_custom_hud_game_mode))
          (`/Engine/EditorBlueprintResources/StandardMacros.IncrementInt` _output_get
            (:`  `
              (`/Game/GameCore/GameMode/BP_CustomHUD_GameMode.IncreaseDamagePerKills` _asbp_custom_hud_game_mode)
              (`|SpawnActorFromClass` "/Game/Systems/SkillTree/BP_Actor/BP_EXP.BP_EXP_C" (`self.GetTransform`) "Undefined" "OverrideRootScale" null null))))
        (:`then_1`
          (`|SpawnActorFromClass` (`KismetArrayLibrary.Array_Random` (`self.Loot_Class`)) (`self.GetTransform`) "Undefined" "OverrideRootScale" null null))))))

(event `self.GSCCore.OnHealthChange`
  (params (DeltaValue :type "Float (single-precision)") (EventTags :type "GameplayTagContainer Structure"))
  ;[0.6937 1 0.447] AI Death
  (if (<= (`.ReturnValue` (`AbilitySystemBlueprintLibrary.GetFloatAttributeFromAbilitySystemComponent` (`self.GSCAbilitySystem`) (struct :`AttributeName` "Health" :`Attribute` "/Script/GASCompanion.GSCAttributeSet:Health" :`AttributeOwner` "/Script/CoreUObject.Class'\"/Script/GASCompanion.GSCAttributeSet\"'"))) 0.0)
    (`self.K2_DestroyActor`)))

(event `self.PawnSensing.OnSeePawn`
  (params (Pawn :type "Pawn Object Reference"))
  ;[1 0.7135 0] AI Behavior(Movement And Attack)
  (`|AIMoveTo` self (0.0 0.0 0.0) (`GameplayStatics.GetPlayerCharacter` 0) (`self.AI Range`) true
    (:`OnSuccess`
      (if true
        (set `self.IsAttacking` true)
        (`|PlayMontage` (`self.Mesh`) "/Game/Demo/Examples/Combo/AbilitySystem/Melee/AM_Attack_PrimaryA_Montage.AM_Attack_PrimaryA_Montage" (`.ReturnValue` (`AbilitySystemBlueprintLibrary.GetFloatAttributeFromAbilitySystemComponent` (`self.GSCAbilitySystem`) (struct :`AttributeName` "AttackSpeed" :`Attribute` "/Script/GASCompanionDemo.MainAttributes:AttackSpeed" :`AttributeOwner` "/Script/CoreUObject.Class'\"/Script/GASCompanionDemo.MainAttributes\"'")))
          (:`OnCompleted`
            (`KismetSystemLibrary.Delay` 0.1)
            (set `self.IsAttacking` false)))))))

(event `self.Sphere.OnComponentBeginOverlap`
  (params (OverlappedComponent :type "PrimitiveComponent Object Reference") (OtherActor :type "Actor Object Reference") (OtherComp :type "PrimitiveComponent Object Reference") (OtherBodyIndex :type Integer) (bFromSweep :type Boolean) (SweepResult :type "HitResult Structure (by ref)"))
  (bind _returnvalue (`AbilitySystemBlueprintLibrary.GetAbilitySystemComponent` OtherActor))
  (if (and (`KismetSystemLibrary.IsValid` _returnvalue) (`self.ActorHasTag` OtherActor "Player") (`self.IsAttacking`))
    (`AbilitySystemComponent.BP_ApplyGameplayEffectToTarget` :`self` (`self.GSCAbilitySystem`) :`GameplayEffectClass` "/Game/GAS/GameplayEffects/CharacterEffects/GE_ApplyDamage.GE_ApplyDamage_C" :`Target` _returnvalue)
    (bind _result (`/Engine/EditorBlueprintResources/StandardMacros.IncrementInt` (`self.Counter`))
      (:`  `
        (bind _output_get (set `self.Counter` _result))
        (`KismetSystemLibrary.PrintString` (`KismetStringLibrary.Conv_IntToString` _output_get))))
    (else
      (`KismetSystemLibrary.PrintString` "Hello"))))

(fn `AI Auto Attack(Melee)`
  (bind _capsulecomponent (`self.CapsuleComponent`))
  (bind _returnvalue (+ (`SceneComponent.K2_GetComponentLocation` _capsulecomponent) (0.0 0.0 90.0)))
  (bind _outhit (`KismetSystemLibrary.LineTraceSingle` _returnvalue (+ _returnvalue (* (`SceneComponent.GetForwardVector` _capsulecomponent) 100.0)) "TraceTypeQuery2"))
  (bind (_bblockinghit _binitialoverlap _time _distance _location _impactpoint _normal _impactnormal _physmat _hitactor) (`GameplayStatics.BreakHitResult` _outhit))
  (if (`KismetSystemLibrary.DoesImplementInterface` _hitactor "/Game/Data/BP_Interface/BPI_Player.BPI_Player_C")
    (`AbilitySystemComponent.BP_ApplyGameplayEffectToTarget` :`self` (`self.GSCAbilitySystem`) :`GameplayEffectClass` "/Game/GAS/GameplayEffects/CharacterEffects/GE_ApplyDamage.GE_ApplyDamage_C" :`Target` (`AbilitySystemBlueprintLibrary.GetAbilitySystemComponent` _hitactor))))

(fn `UserConstructionScript`)