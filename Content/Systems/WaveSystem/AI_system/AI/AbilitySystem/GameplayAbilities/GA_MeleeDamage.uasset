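; GA_MeleeDamage is a Gameplay Ability in the wave system's AI, meant to deal melee damage to the player.
; On activation it casts player character 0 to BP_AI, printing a debug string if that fails.
; It traces on Visibility along the mesh's forward vector for AIAttackRange, with debug drawing.
; A hit actor tagged Player receives ApplyGameplayEffectToTarget from the AI's ability system component, with no effect specified.
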(event `self.K2_ActivateAbility`
  (bind _asbp_ai (cast `/Game/Systems/WaveSystem/AI_system/AI/AI_Parent/BP_AI` (`GameplayStatics.GetPlayerCharacter` 0))
    (:`then`
      (bind _mesh (`Character.Mesh` _asbp_ai))
      (bind _returnvalue (`SceneComponent.K2_GetComponentLocation` _mesh))
      (bind _outhit (`KismetSystemLibrary.LineTraceSingle` :`Start` _returnvalue :`End` (+ _returnvalue (* (`SceneComponent.GetForwardVector` _mesh) (`self.AIAttackRange`))) :`TraceChannel` "TraceTypeQuery1" :`DrawDebugType` "ForDuration"))
      (bind (_bblockinghit _binitialoverlap _time _distance _location _impactpoint _normal _impactnormal _physmat _hitactor) (`GameplayStatics.BreakHitResult` _outhit))
      (if (`Actor.ActorHasTag` _hitactor "Player")
        (`AbilitySystemComponent.BP_ApplyGameplayEffectToTarget` :`self` (`AbilitySystemBlueprintLibrary.GetAbilitySystemComponent` _asbp_ai) :`Target` (`AbilitySystemBlueprintLibrary.GetAbilitySystemComponent` _hitactor))))
    (:`CastFailed`
      (`KismetSystemLibrary.PrintString` "Hello"))))