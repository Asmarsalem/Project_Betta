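; BP_Ranged_AI is a ranged enemy AI Blueprint that fires BP_AIArrow projectiles.
; Shoot spawns a scaled-up arrow at an offset from the Arrow1 component, aligned to the actor's rotation.
; A stored game-time stamp enforces a fixed cooldown between shots, with an attack speed attribute noted as still to be added.
; StopShoot is an empty event marked as still in use.
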(event `StopShoot`
  ;[0 1 0.09742] Shooting system
  ;;[0.9948 0.1068 0] Dont Delete This is an Active Event
)

(event `Shoot`
  (bind _returnvalue (`KismetSystemLibrary.GetGameTimeInSeconds`))
  (bind _returnvalue_2 (`self.K2_GetActorRotation`))
  (bind _xshoot (`self.XShoot`))
  ;[0 1 0.09742] Shooting system
  (if (== _xshoot 0.0)
    (set `self.XShoot` _returnvalue :!label _label)
    (`|SpawnActorFromClass` "/Game/BP_Actors/BP_AIArrow.BP_AIArrow_C" (`KismetMathLibrary.MakeTransform` (+ (`SceneComponent.K2_GetComponentLocation` (`self.Arrow1`)) (`KismetMathLibrary.GreaterGreater_VectorRotator` (-40.0 0.0 0.0) _returnvalue_2)) _returnvalue_2 (2.0 2.0 2.0)) "Undefined" "OverrideRootScale" null null)
    (elif (not (> (+ _xshoot 0.9) _returnvalue))
      (goto _label))))

(fn `UserConstructionScript`)