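; Base enemy AI character for the wave system, using the GSC Ability System for health and movement speed, which it refreshes every tick.
; It is destroyed at zero health, and EndPlay on authority updates the game mode's per-kill damage bonus and spawns experience plus random loot.
; Attack plays a montage with a notify-driven sphere trace that only prints hit results.
; The line-trace melee damage effect and attack-speed timing are unwired.
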(event `self.ReceiveBeginPlay`
  ;[0.00947 0 1] Begin
  (`GameplayStatics.SpawnEmitterAtLocation` "/Game/MapAssets/InfinityBladeEffects/Effects/FX_Mobile/ICE/combat/P_YoYo_IceBlast_Axe_00.P_YoYo_IceBlast_Axe_00" (`self.K2_GetActorLocation` self)))

(event `Set Movement Speed`
  ;[0.03109 0 0.3594] Set AI Movement Speed
  (set `CharacterMovementComponent.MaxWalkSpeed` (`.ReturnValue` (`AbilitySystemBlueprintLibrary.GetFloatAttributeFromAbilitySystemComponent` (`self.GSCAbilitySystem`) (struct :`AttributeName` "Speed" :`Attribute` "/Script/GASCompanionDemo.MainAttributes:Speed" :`AttributeOwner` "/Script/CoreUObject.Class'\"/Script/GASCompanionDemo.MainAttributes\"'"))) (`self.CharacterMovement`)))

(event `Get Number of Starting AI`
  ;[0.2257 1 0.7464] Set Number of Starting AI
  (bind _outactors (`GameplayStatics.GetAllActorsOfClass` "BP_AI_C"))
  (set `self.NumberOfDeployedAI` (`KismetArrayLibrary.Array_Length` _outactors)))

(event `self.ReceiveTick`
  (params (DeltaSeconds :type "Float (single-precision)"))
  ;[1 0.01812 0.6912] EventTick
  (`self.Set Movement Speed`))

(event `Set AI Attack Speed`
  ;[0.03212 1 0] Set AI Attack Speed
  (bind _output_get (set `self.AI Attack Speed` (/ (`.ReturnValue` (`AbilitySystemBlueprintLibrary.GetFloatAttributeFromAbilitySystemComponent` (`self.GSCAbilitySystem`) (struct :`AttributeName` "AttackSpeed" :`Attribute` "/Script/GASCompanionDemo.MainAttributes:AttackSpeed" :`AttributeOwner` "/Script/CoreUObject.Class'\"/Script/GASCompanionDemo.MainAttributes\"'"))) -10.0))))

(event `self.ReceiveEndPlay`
  (params (EndPlayReason :type "EEndPlayReason Enum" :default "Destroyed"))
  ;[0.6939 1 0.4452] AI Death
  (`/Engine/EditorBlueprintResources/ActorMacros.Switch Has Authority`
    (:`Authority`
      (`|ExecutionSequence`
        (:`then_0`
          (bind _asbp_custom_hud_game_mode (cast `/Game/GameCore/GameMode/BP_CustomHUD_GameMode` (`GameplayStatics.GetGameMode`)))
          (bind _output_get (set `/Game/GameCore/GameMode/BP_CustomHUD_GameMode.IncreaseDamagePerKill` 0 _asbp_custom_hud_game_mode))
          (`/Engine/EditorBlueprintResources/StandardMacros.IncrementInt` _output_get
            (:`  `
              (`/Game/GameCore/GameMode/BP_CustomHUD_GameMode.IncreaseDamagePerKills` _asbp_custom_hud_game_mode)
              (`|SpawnActorFromClass` "/Game/Systems/SkillTree/BP_Actor/BP_EXP.BP_EXP_C" (`self.GetTransform`) "Undefined" "OverrideRootScale" null null))))
        (:`then_1`
          (`|SpawnActorFromClass` (`KismetArrayLibrary.Array_Random` (`self.Loot_Class`)) (`self.GetTransform`) "Undefined" "OverrideRootScale" null null))))))

(event `self.GSCCore.OnHealthChange`
  (params (DeltaValue :type "Float (single-precision)") (EventTags :type "GameplayTagContainer Structure"))
  ;[0.6939 1 0.4452] AI Death
  (if (<= (`.ReturnValue` (`AbilitySystemBlueprintLibrary.GetFloatAttributeFromAbilitySystemComponent` (`self.GSCAbilitySystem`) (struct :`AttributeName` "Health" :`Attribute` "/Script/GASCompanion.GSCAttributeSet:Health" :`AttributeOwner` "/Script/CoreUObject.Class'\"/Script/GASCompanion.GSCAttributeSet\"'"))) 0.0)
    (`self.K2_DestroyActor`)))

(event `/Game/Systems/WaveSystem/AI_system/AI/BPI_CombatInterface.Attack`
  (params (AttackSpeed :type "Float (double-precision)"))
  (bind _returnvalue (`SceneComponent.GetSocketLocation` (`self.Mesh`) "hand_rSocket_Begin"))
  ;[0.6939 1 0.4452] Attack player
  (`|PlayMontage` (`self.Mesh`) "/Game/Demo/Examples/Combo/AbilitySystem/Melee/AM_Attack_PrimaryB_Montage.AM_Attack_PrimaryB_Montage"
    (:`OnNotifyBegin`
      (bind (_outhit _returnvalue_2) (`KismetSystemLibrary.SphereTraceSingle` :`Start` _returnvalue :`End` (+ _returnvalue (* (`KismetMathLibrary.GetForwardVector` (`self.K2_GetActorRotation`)) 30.0)) :`Radius` 80.0 :`TraceChannel` "TraceTypeQuery2" :`DrawDebugType` "ForDuration"))
      (if _returnvalue_2
        (`KismetSystemLibrary.PrintString` "Hit")
        (else
          (`KismetSystemLibrary.PrintString` "No hit"))))))

(fn `AI Auto Attack(Melee)`
  (bind _capsulecomponent (`self.CapsuleComponent`))
  (bind _returnvalue (+ (`SceneComponent.K2_GetComponentLocation` _capsulecomponent) (0.0 0.0 90.0)))
  (bind _outhit (`KismetSystemLibrary.LineTraceSingle` _returnvalue (+ _returnvalue (* (`SceneComponent.GetForwardVector` _capsulecomponent) 100.0)) "TraceTypeQuery2"))
  (bind (_bblockinghit _binitialoverlap _time _distance _location _impactpoint _normal _impactnormal _physmat _hitactor) (`GameplayStatics.BreakHitResult` _outhit))
  (if (`KismetSystemLibrary.DoesImplementInterface` _hitactor "/Game/Data/BP_Interface/BPI_Player.BPI_Player_C")
    (`AbilitySystemComponent.BP_ApplyGameplayEffectToTarget` :`self` (`self.GSCAbilitySystem`) :`GameplayEffectClass` "/Game/GAS/GameplayEffects/CharacterEffects/GE_ApplyDamage.GE_ApplyDamage_C" :`Target` (`AbilitySystemBlueprintLibrary.GetAbilitySystemComponent` _hitactor))))

(fn `UserConstructionScript`)