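; BP_EnemyController is an AI controller for enemy NPCs in the wave system.
; On BeginPlay it starts the BT_NPC behavior tree and caches the controlled pawn as BP_AI.
; Perception updates call HandleSightSense, but that function's logic is disconnected and never runs.
; The unused logic would set or clear the player as blackboard TargetActor and store LastKnownLocation when sight is lost.
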(event `self.ReceiveBeginPlay`
  (`self.RunBehaviorTree` "/Game/Systems/WaveSystem/AI_system/AI/AI_Parent/BT_NPC.BT_NPC")
  (bind _asbp_ai (cast `/Game/Systems/WaveSystem/AI_system/AI/AI_Parent/BP_AI` (`self.K2_GetPawn`)))
  (set `self.As BP AI` _asbp_ai)
  (`KismetSystemLibrary.Delay` 3.0))

(event `self.AIPerception.OnTargetPerceptionUpdated`
  (params (Actor :type "Actor Object Reference") (Stimulus :type "AIStimulus Structure"))
  (`self.HandleSightSense` Actor Stimulus))

(fn `HandleSightSense`
  (params (Actor :type "Actor Object Reference") (Stimlus :type "AIStimulus Structure")))

(fn `UserConstructionScript`)