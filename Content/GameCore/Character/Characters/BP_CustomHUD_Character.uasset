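; Player character for a custom HUD example map, built on GAS and GSCCore.
; BeginPlay adds the map's input context and starts looping timers that auto-activate Lightning and Poison abilities; J triggers an AI stun.
; Level attribute changes spawn a level-up widget component, locally in standalone or by multicast to clients.
; Events apply health-regen and death-strike effects, while XP number display and level-up logic are disconnected.
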(event `Key|J`
  (params (Key :type "Key Structure"))
  ;[0.5044 0 1] Abilities To Activate
  (:`Pressed`
    (`AbilitySystemComponent.TryActivateAbilityByClass` (`self.AbilitySystemComponent`) "/Game/GAS/Abilities/Stun/GA_StunAI.GA_StunAI_C" true)))

(event `self.ReceiveBeginPlay`
  ;[0 0 0 0] Begin Play: Add Input Mapping specific to this example map (IA_Ability_01/02)
  (`parent.ReceiveBeginPlay`)
  (bind _asplayer_controller (cast `PlayerController` (`self.GetController`)))
  (`EnhancedInputSubsystemInterface.AddMappingContext` (pcsubsystem `EnhancedInputLocalPlayerSubsystem` _asplayer_controller) "/Game/Demo/Examples/CustomHUD/Inputs/MC_CustomHUD.MC_CustomHUD" 1 (struct))
  (`KismetSystemLibrary.K2_SetTimerDelegate` (delegate `Lightning`) 0.3 true)
  (`KismetSystemLibrary.K2_SetTimerDelegate` (delegate `Poison`) 2.0 true))

(event `Lightning`
  ;[0 0 0 0] Begin Play: Add Input Mapping specific to this example map (IA_Ability_01/02)
  (`AbilitySystemComponent.TryActivateAbilityByClass` (`self.AbilitySystemComponent`) "/Game/GAS/Abilities/Lightning/GA_Lightning.GA_Lightning_C" true))

(event `Poison`
  ;[0 0 0 0] Begin Play: Add Input Mapping specific to this example map (IA_Ability_01/02)
  (`AbilitySystemComponent.TryActivateAbilityByClass` (`self.AbilitySystemComponent`) "/Game/GAS/Abilities/Poison/GA_Poison.GA_Poison_C" true))

(event `self.GSCCoreComponent.OnAttributeChange`
  (params (Attribute :type "GameplayAttribute Structure") (DeltaValue :type "Float (single-precision)") (EventTags :type "GameplayTagContainer Structure"))
  ;[0 0 0 0] On Attribute Change Event: You can react to attribute value changes here, for example to update UI
  (`|SwitchGameplayAttribute` Attribute
    (:`Level`
      (`self.ReplicatedAddLevelUPWC`))))

(event `self.GSCCoreComponent.OnPostGameplayEffectExecute`
  (params (Attribute :type "GameplayAttribute Structure") (SourceActor :type "Actor Object Reference") (TargetActor :type "Actor Object Reference") (SourceTags :type "GameplayTagContainer Structure (by ref)") (Payload :type "GSCGameplayEffectExecuteData Structure"))
  ;[0 0 0 0] Handle XP Change via PostGameplayEffectExecute triggered by AttributeSets
)

(event `Health regeneration`
  (bind _abilitysystemcomponent (`self.AbilitySystemComponent`))
  ;[1 1 1] When wave level increments implement this event
  (`AbilitySystemComponent.BP_ApplyGameplayEffectToTarget` :`self` _abilitysystemcomponent :`GameplayEffectClass` "/Game/GAS/GameplayEffects/AttributesUpgrades/GE_IncreaseHealthRegen.GE_IncreaseHealthRegen_C" :`Target` _abilitysystemcomponent))

(event `AddXPNumberWC`
  (params (Number :type "Float (double-precision)"))
  ;[0 0 0 0] Replicated Add XP Number Component
  (bind _returnvalue (`AddComponent|NODE_AddWC_XP_Text-4` :`bManualAttachment` true :`RelativeTransform` (`self.GetTransform`)))
  (`/Game/UI/UI/WC_XP_Text.SetNumber` _returnvalue Number))

(event `Multicast_AddXPNumberWC`
  (params (Number :type "Float (double-precision)"))
  ;[0 0 0 0] Replicated Add XP Number Component
  (if (not (`KismetSystemLibrary.IsServer`))
    (`self.AddXPNumberWC` Number)))

(event `ReplicatedAddXPNumberWC`
  (params (Number :type "Float (double-precision)"))
  ;[0 0 0 0] Replicated Add XP Number Component
  (if (`KismetSystemLibrary.IsStandalone`)
    (`self.AddXPNumberWC` Number)
    (else
      (`self.Multicast_AddXPNumberWC` Number))))

(event `AddLevelUPWC`
  ;[0 0 0 0] Replicated Add Level Up Widget Component
  (bind _returnvalue (`AddComponent|NODE_AddWC_LevelUp-4` :`bManualAttachment` true :`RelativeTransform` (`self.GetTransform`)))
  (`/Game/UI/UI/WC_LevelUp.SetNumber` _returnvalue 0.0))

(event `Multicast_AddLevelUPWC`
  ;[0 0 0 0] Replicated Add Level Up Widget Component
  (if (not (`KismetSystemLibrary.IsServer`))
    (`self.AddLevelUPWC`)))

(event `ReplicatedAddLevelUPWC`
  ;[0 0 0 0] Replicated Add Level Up Widget Component
  (if (`KismetSystemLibrary.IsStandalone`)
    (`self.AddLevelUPWC`)
    (else
      (`self.Multicast_AddLevelUPWC`))))

(fn `DeathStrikeMain`
  (params (`Ability System Component` :type "AbilitySystemComponent Object Reference"))
  (`AbilitySystemComponent.BP_ApplyGameplayEffectToTarget` :`self` (`self.AbilitySystemComponent`) :`GameplayEffectClass` "/Game/GAS/GameplayEffects/CharacterEffects/GE_DeathStrike.GE_DeathStrike_C" :`Target` `Ability System Component` :`Level` (`.ReturnValue` (`AbilitySystemBlueprintLibrary.GetFloatAttributeFromAbilitySystemComponent` `Ability System Component` (struct :`AttributeName` "DeathStrike" :`Attribute` "/Script/GASCompanionDemo.MainAttributes:DeathStrike" :`AttributeOwner` "/Script/CoreUObject.Class'\"/Script/GASCompanionDemo.MainAttributes\"'")))))

(fn `DisplayXPNumber`
  (params (Number :type "Float (double-precision)")))

(fn `HandleXPChange`
  (params (DeltaValue :type "Float (double-precision)"))
  (locals (CurrentXP :type "Float (double-precision)" :default 0.0) (NextLevelXP :type "Float (double-precision)" :default 0.0))
  ;[0.4623 1 0.8065] Level Up
)

(fn `UserConstructionScript`)