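; BP_Minions is a minion pawn for the Mage character that chases a BP_AI actor and damages what it hits.
; Each Tick it looks up a BP_AI, issues AIMoveTo toward it and calls AttackAI immediately, without waiting for arrival.
; AttackAI runs a short debug-drawn object trace forward from Arrow1, ignoring the player.
; Hit actors with an ability system component receive GE_ApplyDamage through GSCAbilitySystem, with no cooldown.
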(event `self.ReceiveTick`
  (params (DeltaSeconds :type "Float (single-precision)"))
  (bind _returnvalue (`GameplayStatics.GetActorOfClass` "/Game/Systems/WaveSystem/AI_system/AI/BP_AI.BP_AI_C"))
  (`|AIMoveTo` self (`SceneComponent.K2_GetComponentLocation` (`Character.Mesh` _returnvalue)) _returnvalue 10.0
    (:`then`
      (`self.AttackAI`))))

(fn `AttackAI`
  (bind _arrow1 (`self.Arrow1`))
  (bind _returnvalue (`SceneComponent.K2_GetComponentLocation` _arrow1))
  (bind _outhit (`KismetSystemLibrary.LineTraceSingleForObjects` _returnvalue (+ _returnvalue (* (`SceneComponent.GetForwardVector` _arrow1) 300.0)) (`|MakeArray` "ObjectTypeQuery9" :!type "EObjectTypeQuery Enum") false (`|MakeArray` (`GameplayStatics.GetPlayerCharacter` 0) :!type "Actor Object Reference") "ForDuration"))
  (bind _returnvalue_2 (`AbilitySystemBlueprintLibrary.GetAbilitySystemComponent` (`.HitActor` (`GameplayStatics.BreakHitResult` _outhit))))
  (if (`KismetSystemLibrary.IsValid` _returnvalue_2)
    (`AbilitySystemComponent.BP_ApplyGameplayEffectToTarget` :`self` (`self.GSCAbilitySystem`) :`GameplayEffectClass` "/Game/GAS/GameplayEffects/CharacterEffects/GE_ApplyDamage.GE_ApplyDamage_C" :`Target` _returnvalue_2)))

(fn `UserConstructionScript`)