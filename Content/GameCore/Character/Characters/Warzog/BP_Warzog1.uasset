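; Warzog character Blueprint that restores its skeletal mesh from the "SK" save slot on BeginPlay and tracks left mouse hold in a rotation flag.
; XP number and level-up widget components spawn at the actor through wrappers that run locally in standalone or multicast, skipping the server.
; Helpers play a melee montage and self-apply the critical damage GameplayEffect at an attribute-derived level; SetAttackRange is an empty stub.
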(event `self.ReceiveBeginPlay`
  (bind _returnvalue (`GameplayStatics.DoesSaveGameExist` "SK"))
  (if _returnvalue
    (bind _returnvalue_2 (`GameplayStatics.LoadGameFromSlot` "SK"))
    (bind _assg_new_save_game (cast `/Game/Data/SaveGame/SG_NewSaveGame` _returnvalue_2))
    (`SkeletalMeshComponent.SetSkeletalMeshAsset` (`self.Mesh`) (`/Game/Data/SaveGame/SG_NewSaveGame.SKELETAL MESH` _assg_new_save_game))))

(event `Key|LeftMouseButton`
  (params (Key :type "Key Structure"))
  (:`Pressed`
    (set `self.ROTATION` true))
  (:`Released`
    (set `self.ROTATION` false)))

(event `AddXPNumberWC`
  (params (Number :type "Float (double-precision)"))
  ;[0 0 0 0] Replicated Add XP Number Component
  (bind _returnvalue (`AddComponent|NODE_AddWC_XP_Text-4` :`bManualAttachment` true :`RelativeTransform` (`self.GetTransform`)))
  (`/Game/UI/UI/WC_XP_Text.SetNumber` _returnvalue Number))

(event `Multicast_AddXPNumberWC`
  (params (Number :type "Float (double-precision)"))
  ;[0 0 0 0] Replicated Add XP Number Component
  (if (not (`KismetSystemLibrary.IsServer`))
    (`self.AddXPNumberWC` Number)))

(event `ReplicatedAddXPNumberWC`
  (params (Number :type "Float (double-precision)"))
  ;[0 0 0 0] Replicated Add XP Number Component
  (if (`KismetSystemLibrary.IsStandalone`)
    (`self.AddXPNumberWC` Number)
    (else
      (`self.Multicast_AddXPNumberWC` Number))))

(event `AddLevelUPWC`
  ;[0 0 0 0] Replicated Add Level Up Widget Component
  (bind _returnvalue (`AddComponent|NODE_AddWC_LevelUp-4` :`bManualAttachment` true :`RelativeTransform` (`self.GetTransform`)))
  (`/Game/UI/UI/WC_LevelUp.SetNumber` _returnvalue 0.0))

(event `Multicast_AddLevelUPWC`
  ;[0 0 0 0] Replicated Add Level Up Widget Component
  (if (not (`KismetSystemLibrary.IsServer`))
    (`self.AddLevelUPWC`)))

(event `ReplicatedAddLevelUPWC`
  ;[0 0 0 0] Replicated Add Level Up Widget Component
  (if (`KismetSystemLibrary.IsStandalone`)
    (`self.AddLevelUPWC`)
    (else
      (`self.Multicast_AddLevelUPWC`))))

(fn `CriticalDamage & CriticalChance`
  (params (`Ability System Component` :type "AbilitySystemComponent Object Reference"))
  (bind _abilitysystemcomponent (`self.AbilitySystemComponent`))
  (`AbilitySystemComponent.BP_ApplyGameplayEffectToTarget` :`self` _abilitysystemcomponent :`GameplayEffectClass` "/Game/GAS/GameplayEffects/CharacterEffects/GE_CriticalDamage.GE_CriticalDamage_C" :`Target` `Ability System Component` :`Level` (`KismetMathLibrary.Conv_IntToDouble` (`KismetMathLibrary.FTrunc` (`.ReturnValue` (`AbilitySystemBlueprintLibrary.GetFloatAttributeFromAbilitySystemComponent` _abilitysystemcomponent (struct :`AttributeName` "CriticalChance" :`Attribute` "/Script/GASCompanionDemo.MainAttributes:CriticalChance" :`AttributeOwner` "/Script/CoreUObject.Class'\"/Script/GASCompanionDemo.MainAttributes\"'")))))))

(fn `Melee Shoot`
  (params (CharacterAnimation :type "AnimMontage Object Reference"))
  (`self.PlayAnimMontage` CharacterAnimation 1.5))

(fn `Set Attack Range`
  (params (AttackRange :type "Float (double-precision)")))

(fn `UserConstructionScript`)