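; Playable Warzog character built on the Gameplay Ability System with GSC companion components, adding an input mapping context on BeginPlay.
; Walk speed follows an attribute every tick, and a KnockBack event activates its ability on every seventh click.
; XP changes trigger number display and XP handling, while level changes spawn a level-up widget, multicast to non-server instances outside standalone.
; Helper functions play melee montages and apply the critical damage effect.
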(event `Movement speed`
  ;[0.02433 0 1] Set  Movement Speed
  (set `CharacterMovementComponent.MaxWalkSpeed` (`.ReturnValue` (`AbilitySystemBlueprintLibrary.GetFloatAttributeFromAbilitySystemComponent` (`self.AbilitySystemComponent`) (struct :`AttributeName` "Speed" :`Attribute` "/Script/GASCompanionDemo.MainAttributes:Speed" :`AttributeOwner` "/Script/CoreUObject.Class'\"/Script/GASCompanionDemo.MainAttributes\"'"))) (`self.CharacterMovement`)))

(event `self.ReceiveTick`
  (params (DeltaSeconds :type "Float (single-precision)"))
  ;[0.02433 0 1] Set  Movement Speed
  (`self.Movement speed`))

(event `self.ReceiveBeginPlay`
  ;[0 0 0 0] Begin Play: Add Input Mapping specific to this example map (IA_Ability_01/02)
  (`parent.ReceiveBeginPlay`)
  (bind _asplayer_controller (cast `PlayerController` (`self.GetController`)))
  (`EnhancedInputSubsystemInterface.AddMappingContext` (pcsubsystem `EnhancedInputLocalPlayerSubsystem` _asplayer_controller) "/Game/Demo/Examples/CustomHUD/Inputs/MC_CustomHUD.MC_CustomHUD" 1 (struct)))

(event `self.GSCCoreComponent.OnAttributeChange`
  (params (Attribute :type "GameplayAttribute Structure") (DeltaValue :type "Float (single-precision)") (EventTags :type "GameplayTagContainer Structure"))
  ;[0 0 0 0] On Attribute Change Event: You can react to attribute value changes here, for example to update UI
  (`|SwitchGameplayAttribute` Attribute
    (:`Level`
      (`self.ReplicatedAddLevelUPWC`))))

(event `self.GSCCoreComponent.OnPostGameplayEffectExecute`
  (params (Attribute :type "GameplayAttribute Structure") (SourceActor :type "Actor Object Reference") (TargetActor :type "Actor Object Reference") (SourceTags :type "GameplayTagContainer Structure (by ref)") (Payload :type "GSCGameplayEffectExecuteData Structure"))
  (bind (_attributeset _abilitysystemcomponent _deltavalue) (break `GSCGameplayEffectExecuteData` Payload))
  ;[0 0 0 0] Handle XP Change via PostGameplayEffectExecute triggered by AttributeSets
  (`|SwitchGameplayAttribute` Attribute
    (:`CurrentXP`
      (`self.DisplayXPNumber` _deltavalue)
      (`self.HandleXPChange` _deltavalue))))

(event `KnockBack`
  ;[1 0.6955 0.3496] KnockBack Ability
  (if (== (mod (`self.NbOfClicks`) 7) 0)
    (`AbilitySystemComponent.TryActivateAbilityByClass` (`self.AbilitySystemComponent`) "/Game/GAS/Abilities/KnockBack/GA_KnockBack.GA_KnockBack_C" true)))

(event `AddXPNumberWC`
  (params (Number :type "Float (double-precision)"))
  ;[0 0 0 0] Replicated Add XP Number Component
  (bind _returnvalue (`AddComponent|NODE_AddWC_XP_Text-4` :`bManualAttachment` true :`RelativeTransform` (`self.GetTransform`)))
  (`/Game/UI/UI/WC_XP_Text.SetNumber` _returnvalue Number))

(event `Multicast_AddXPNumberWC`
  (params (Number :type "Float (double-precision)"))
  ;[0 0 0 0] Replicated Add XP Number Component
  (if (not (`KismetSystemLibrary.IsServer`))
    (`self.AddXPNumberWC` Number)))

(event `ReplicatedAddXPNumberWC`
  (params (Number :type "Float (double-precision)"))
  ;[0 0 0 0] Replicated Add XP Number Component
  (if (`KismetSystemLibrary.IsStandalone`)
    (`self.AddXPNumberWC` Number)
    (else
      (`self.Multicast_AddXPNumberWC` Number))))

(event `AddLevelUPWC`
  ;[0 0 0 0] Replicated Add Level Up Widget Component
  (bind _returnvalue (`AddComponent|NODE_AddWC_LevelUp-4` :`bManualAttachment` true :`RelativeTransform` (`self.GetTransform`)))
  (`/Game/UI/UI/WC_LevelUp.SetNumber` _returnvalue 0.0))

(event `Multicast_AddLevelUPWC`
  ;[0 0 0 0] Replicated Add Level Up Widget Component
  (if (not (`KismetSystemLibrary.IsServer`))
    (`self.AddLevelUPWC`)))

(event `ReplicatedAddLevelUPWC`
  ;[0 0 0 0] Replicated Add Level Up Widget Component
  (if (`KismetSystemLibrary.IsStandalone`)
    (`self.AddLevelUPWC`)
    (else
      (`self.Multicast_AddLevelUPWC`))))

(fn `CriticalDamage & CriticalChance`
  (params (`Ability System Component` :type "AbilitySystemComponent Object Reference"))
  (bind _abilitysystemcomponent (`self.AbilitySystemComponent`))
  (`AbilitySystemComponent.BP_ApplyGameplayEffectToTarget` :`self` _abilitysystemcomponent :`GameplayEffectClass` "/Game/GAS/GameplayEffects/CharacterEffects/GE_CriticalDamage.GE_CriticalDamage_C" :`Target` `Ability System Component` :`Level` (`KismetMathLibrary.Conv_IntToDouble` (`KismetMathLibrary.FTrunc` (`.ReturnValue` (`AbilitySystemBlueprintLibrary.GetFloatAttributeFromAbilitySystemComponent` _abilitysystemcomponent (struct :`AttributeName` "CriticalChance" :`Attribute` "/Script/GASCompanionDemo.MainAttributes:CriticalChance" :`AttributeOwner` "/Script/CoreUObject.Class'\"/Script/GASCompanionDemo.MainAttributes\"'")))))))

(fn `Melee Shoot`
  (params (CharacterAnimation :type "AnimMontage Object Reference"))
  (`self.PlayAnimMontage` CharacterAnimation 1.5))

(fn `UserConstructionScript`)