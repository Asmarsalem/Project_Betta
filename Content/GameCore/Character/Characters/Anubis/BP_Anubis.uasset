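; BP_Anubis is the Anubis character Blueprint, with debug-style key inputs for AI movement and an ability.
; Pressing F casts its controller to BP_EnemyController and stops its movement.
; Pressing M activates the GA_SkullBreak gameplay ability through the Ability System Component.
; BeginPlay, Tick and the construction script only call their parent implementations.
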(event `Key|F`
  (params (Key :type "Key Structure"))
  (:`Pressed`
    (bind _asbp_enemy_controller (cast `/Game/Systems/WaveSystem/AI_system/AI/BP_EnemyController` (`self.GetController`)))
    (`Controller.StopMovement` _asbp_enemy_controller)))

(event `self.ReceiveBeginPlay`
  (`parent.ReceiveBeginPlay`))

(event `self.ReceiveTick`
  (params (DeltaSeconds :type "Float (single-precision)"))
  (`parent.ReceiveTick` 0.0))

(event `Key|M`
  (params (Key :type "Key Structure"))
  (:`Pressed`
    (`AbilitySystemComponent.TryActivateAbilityByClass` (`self.AbilitySystemComponent`) "/Game/GAS/Abilities/SkullBreak/GA_SkullBreak.GA_SkullBreak_C" true)))

(fn `UserConstructionScript`
  (`parent.UserConstructionScript`))