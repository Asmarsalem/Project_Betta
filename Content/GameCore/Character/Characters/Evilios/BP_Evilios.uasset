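; Evilios is a playable ranged character that fires arrows, built on the Gameplay Ability System and a UACEvilios component.
; BeginPlay configures that component with arrow, ricochet, multi-arrow and enemy settings.
; Each Tick copies an ability-system attribute into walk speed and runs the component's AutoAim, while V activates the multi-arrow ability.
; A helper applies an attribute-levelled critical damage effect; click-counting auto-shoot and attack-range logic are disconnected.
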(event `Set MovementSpeed`
  ;[0 0.7647 1] Set Movement Speed
  (set `CharacterMovementComponent.MaxWalkSpeed` (`.ReturnValue` (`AbilitySystemBlueprintLibrary.GetFloatAttributeFromAbilitySystemComponent` (`self.AbilitySystemComponent`) (struct :`AttributeName` "Speed" :`Attribute` "/Script/GASCompanionDemo.MainAttributes:Speed" :`AttributeOwner` "/Script/CoreUObject.Class'\"/Script/GASCompanionDemo.MainAttributes\"'"))) (`self.CharacterMovement`)))

(event `self.ReceiveBeginPlay`
  ;[1 0 0.01747] Set Attack Range
  (`parent.ReceiveBeginPlay`)
  (`self.Init`))

(event `self.ReceiveTick`
  (params (DeltaSeconds :type "Float (single-precision)"))
  (`|ExecutionSequence`
    (:`then_0`
      (`self.Set MovementSpeed`))
    (:`then_1`
      (`UAC_Evilios.AutoAim` (`self.UAC_Evilios`)))))

(event `Key|V`
  (params (Key :type "Key Structure"))
  ;[0.3586 1 0] Activate Abilities By Input
  (:`Pressed`
    (`AbilitySystemComponent.TryActivateAbilityByClass` (`self.AbilitySystemComponent`) "/Game/GAS/Abilities/MultiArrows/GA_MultiArrows.GA_MultiArrows_C" true)))

(event `Key|LeftMouseButton`
  (params (Key :type "Key Structure"))
  ;[0 0.05173 1] Abilities to Activate
)

(fn `CriticalDamage & CriticalChance`
  (params (AbilitySystemComponent :type "AbilitySystemComponent Object Reference"))
  (bind _abilitysystemcomponent (`self.AbilitySystemComponent`))
  (`AbilitySystemComponent.BP_ApplyGameplayEffectToTarget` :`self` _abilitysystemcomponent :`GameplayEffectClass` "/Game/GAS/GameplayEffects/CharacterEffects/GE_CriticalDamage.GE_CriticalDamage_C" :`Target` AbilitySystemComponent :`Level` (`KismetMathLibrary.Conv_IntToDouble` (`KismetMathLibrary.FTrunc` (`.ReturnValue` (`AbilitySystemBlueprintLibrary.GetFloatAttributeFromAbilitySystemComponent` _abilitysystemcomponent (struct :`AttributeName` "CriticalChance" :`Attribute` "/Script/GASCompanionDemo.MainAttributes:CriticalChance" :`AttributeOwner` "/Script/CoreUObject.Class'\"/Script/GASCompanionDemo.MainAttributes\"'")))))))

(fn `Init`
  (bind _uac_evilios (`self.UAC_Evilios`))
  (set `UAC_Evilios.SingleArrow` "/Game/BP_Actors/BP_Arrow.BP_Arrow_C" _uac_evilios)
  (set `UAC_Evilios.EnemyClass` "/Game/Systems/WaveSystem/AI_system/AI/BP_AI.BP_AI_C" _uac_evilios)
  (set `UAC_Evilios.RecochetArrow` "/Game/BP_Actors/BP_Recochet_Arrorw.BP_Recochet_Arrorw_C" _uac_evilios)
  (set `UAC_Evilios.MultiArrowsIndex` 3 _uac_evilios)
  (set `UAC_Evilios.RecochetCoolDown` 4.0 _uac_evilios)
  (set `UAC_Evilios.MultiArrow` "/Game/GAS/Abilities/MultiArrows/GA_MultiArrows.GA_MultiArrows_C" _uac_evilios)
  (`KismetSystemLibrary.PrintString` "Hello" true true (struct :`R` 0.493941 :`G` 0.365314 :`B` 1.0 :`A` 1.0)))

(fn `UserConstructionScript`
  (`parent.UserConstructionScript`))