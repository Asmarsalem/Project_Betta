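; Arrow actor for the Evilios character that damages enemies through the Gameplay Ability System.
; On box overlap with a BPI_Enemy actor that has an ability system component, it applies GE_ApplyDamage from player 0's component, then destroys itself.
; A KnockBackAbility event activates GA_KnockBack on the player when the game mode's click count is a multiple of ten.
; An unfinished Ricochet function, meant to spawn further arrows, is never run.
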(event `KnockBack Ability`
  ;[0 0.1388 1] KnockBack Ability
  (bind _asbp_custom_hud_game_mode (cast `/Game/GameCore/GameMode/BP_CustomHUD_GameMode` (`GameplayStatics.GetGameMode`)))
  (if (== (mod (`/Game/GameCore/GameMode/BP_CustomHUD_GameMode.NbOfClicks` _asbp_custom_hud_game_mode) 10) 0)
    (bind _asbp_evilios (cast `/Game/GameCore/Character/Characters/Evilios/BP_Evilios` (`GameplayStatics.GetPlayerCharacter` 0)))
    (`AbilitySystemComponent.TryActivateAbilityByClass` (`GSCModularCharacter.AbilitySystemComponent` _asbp_evilios) "/Game/GAS/Abilities/KnockBack/GA_KnockBack.GA_KnockBack_C" true)))

(event `self.Box.OnComponentBeginOverlap`
  (params (OverlappedComponent :type "PrimitiveComponent Object Reference") (OtherActor :type "Actor Object Reference") (OtherComp :type "PrimitiveComponent Object Reference") (OtherBodyIndex :type Integer) (bFromSweep :type Boolean) (SweepResult :type "HitResult Structure (by ref)"))
  (bind _returnvalue (`AbilitySystemBlueprintLibrary.GetAbilitySystemComponent` OtherActor))
  ;[1 0.935 0] Apply Damage to Enemies and destroy Arrow
  (if (and (`KismetSystemLibrary.DoesImplementInterface` OtherActor "/Game/Data/BP_Interface/BPI_Enemy.BPI_Enemy_C") (`KismetSystemLibrary.IsValid` _returnvalue))
    (bind _asbp_evilios (cast `/Game/GameCore/Character/Characters/Evilios/BP_Evilios` (`GameplayStatics.GetPlayerCharacter` 0)))
    (`AbilitySystemComponent.BP_ApplyGameplayEffectToTarget` :`self` (`AbilitySystemBlueprintLibrary.GetAbilitySystemComponent` _asbp_evilios) :`GameplayEffectClass` "/Game/GAS/GameplayEffects/CharacterEffects/GE_ApplyDamage.GE_ApplyDamage_C" :`Target` _returnvalue)
    (if (`KismetSystemLibrary.DoesImplementInterface` OtherActor "/Game/Data/BP_Interface/BPI_Enemy.BPI_Enemy_C")
      (`self.K2_DestroyActor`))))

(fn `Ricochet`
  (params (`Other Actor` :type "Actor Object Reference"))
  (if (and (`self.ActorHasTag` `Other Actor` "Enemy") (`KismetSystemLibrary.IsValid` (`AbilitySystemBlueprintLibrary.GetAbilitySystemComponent` `Other Actor`)))
    (for _ (range 3)
      (bind _returnvalue (`GameplayStatics.GetActorOfClass` "/Game/Systems/WaveSystem/AI_system/AI/BP_AI.BP_AI_C"))
      (bind _returnvalue_2 (`SceneComponent.K2_GetComponentLocation` (`Actor.RootComponent` _returnvalue)))
      (`|SpawnActorFromClass` "BP_EviliosArrow_C" (`KismetMathLibrary.MakeTransform` _returnvalue_2 (`KismetMathLibrary.FindLookAtRotation` _returnvalue_2 _returnvalue_2)) "Undefined" "OverrideRootScale" null null))
    (`KismetSystemLibrary.PrintString` "Hello")
    (else
      (`KismetSystemLibrary.PrintString` "Not Detected"))))

(fn `UserConstructionScript`)