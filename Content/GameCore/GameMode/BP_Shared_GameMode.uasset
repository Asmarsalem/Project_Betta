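; Shared Game Mode Blueprint that handles respawning player pawns at a given transform.
; TryRespawnPawn calls RespawnActor, which caches the pawn's PlayerController, destroys the pawn, then calls SpawnActor if the cached controller is valid.
; The SpawnActor event spawns a new pawn of the same class, adjusting for collisions but always spawning, and has the controller possess it.
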(event `SpawnActor`
  (params (PawnClass :type "Pawn Class Reference") (SpawnTransform :type "Transform Structure") (PC :type "PlayerController Object Reference"))
  ;[0.491 0.7011 0.09084 0.25] Spawn Actor (for respawn)
  (bind _returnvalue (`|SpawnActorFromClass` PawnClass SpawnTransform "AdjustIfPossibleButAlwaysSpawn" "OverrideRootScale" null null))
  (`Controller.Possess` PC _returnvalue))

(event `/Game/Demo/Shared/Core/BPI_GameMode.TryRespawnPawn`
  (params (Pawn :type "Pawn Object Reference") (SpawnTransform :type "Transform Structure"))
  ;[0.491 0.7011 0.09084 0.25] Spawn Actor (for respawn)
  (`self.RespawnActor` Pawn null SpawnTransform))

(fn `RespawnActor`
  (params (InPawn :type "Pawn Object Reference") (InCharacter :type "GSCModularCharacter Object Reference") (InSpawnTransform :type "Transform Structure"))
  (locals (LocalPlayerController :type "PlayerController Object Reference"))
  (`|ExecutionSequence`
    (:`then_0`
      ;[0 0 0 0] Store Ref to PC before destroying actor
      (bind _asplayer_controller (cast `PlayerController` (`Pawn.GetController` (`local.InPawn`))))
      (set `local.LocalPlayerController` _asplayer_controller))
    (:`then_1`
      (`self.K2_DestroyActor` (`local.InPawn`)))
    (:`then_2`
      (bind _localplayercontroller (`local.LocalPlayerController`)
        (:`then`
          (`self.SpawnActor` (`GameplayStatics.GetObjectClass` (`local.InPawn`)) (`local.InSpawnTransform`) _localplayercontroller))
        (:`else`)))))

(fn `UserConstructionScript`)