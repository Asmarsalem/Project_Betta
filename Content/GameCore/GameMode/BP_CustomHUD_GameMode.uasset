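; Game mode for a top-down shooter that handles player spawning, AI waves and shared XP through the Gameplay Ability System.
; PostLogin spawns BP_Evilios, leaving the loaded save's hero unused.
; Helpers cycle through waves, spawn AI at reachable points, and apply XP and kill-based damage effects; BeginPlay is empty.
; XP attribute changes and level-ups are pushed to every player's pawn through a PlayerArray loop.
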(event `self.K2_PostLogin`
  (params (NewPlayer :type "PlayerController Object Reference"))
  ;[0 1 0.3589] Spawn Character On Begin To Play
  (bind _aspc_top_down_shooter (cast `PC_TopDownShooter` NewPlayer))
  (`self.SpawnCharacter` _aspc_top_down_shooter))

(event `IncreaseDamagePerKills`
  (bind _previouskillvalue (`self.PreviousKillValue`))
  ;[1 0 0.2967] Salim Code (Check Later)
  (bind _asbp_anubis (cast `/Game/GameCore/Character/Characters/Anubis/BP_Anubis` (`GameplayStatics.GetPlayerCharacter` 0)))
  (if (> (`self.IncreaseDamagePerKill`) _previouskillvalue)
    (`AbilitySystemComponent.BP_ApplyGameplayEffectToSelf` :`self` (`AbilitySystemBlueprintLibrary.GetAbilitySystemComponent` _asbp_anubis) :`GameplayEffectClass` "/Game/GAS/GameplayEffects/CharacterEffects/GE_IncreaseDamage.GE_IncreaseDamage_C")
    (bind _result (`/Engine/EditorBlueprintResources/StandardMacros.IncrementInt` _previouskillvalue)
      (:`  `
        (set `self.PreviousKillValue` _result)))))

(event `self.SpawnAiHandle`
  ;[0.4748 0.1691 1] Wave System Handle
)

(event `self.ReceiveBeginPlay`
  ;[0.121 0.43 1] Begin to Play
)

(event `GetNumberOfStartingAI`
  ;[1 0 0.2967] Salim Code (Check Later)
  (bind _outactors (`GameplayStatics.GetAllActorsOfClass` "/Game/Systems/WaveSystem/AI_system/AI/BP_AI.BP_AI_C"))
  (set `self.NumberOfDeployedAI` (`KismetArrayLibrary.Array_Length` _outactors)))

(event `self.GSCCoreComponent.OnAttributeChange`
  (params (Attribute :type "GameplayAttribute Structure") (DeltaValue :type "Float (single-precision)") (EventTags :type "GameplayTagContainer Structure"))
  ;[1 0.02677 0] Bind On Attributes Change
  (`self.OnAttributesChange` Attribute))

(fn `ADDXP`
  (`AbilitySystemComponent.BP_ApplyGameplayEffectToSelf` :`self` (`self.GSCAbilitySystem`) :`GameplayEffectClass` "/Game/Systems/SkillTree/GE_EFffects/GE_ADDXP.GE_ADDXP_C"))

(fn `AiChance`
  (bind _returnvalue (`|GetDataTableRow` "/Game/UI/Widget/TABLES/DT_AIChance.DT_AIChance" "1")))

(fn `BindOnLevelChange`
  (params (CurrentXp :type "Float (single-precision)") (MaxXP :type "Float (single-precision)") (Level :type "Float (single-precision)"))
  (bind _asbp_custom_hud_character (`self.GetAllpPawnsRef`)
    (:`LoopBody`
      (`/Game/Systems/SkillTree/AC_SkillsTree.ExecuteLevelUP` (`/Game/GameCore/Character/Characters/BP_CustomHUD_Character.AC_SkillsTree` _asbp_custom_hud_character)))))

(fn `SpawnAi`
  (params (Value :type "Float (double-precision)"))
  (returns (Success :type Boolean))
  (locals (ValueRef :type "Float (double-precision)"))
  (bind (_success _returnvalue) (`self.GetRandomReachableLocation` "/Game/GameCore/Character/Characters/BP_CustomHUD_Character.BP_CustomHUD_Character_C"))
  (set `local.ValueRef` Value)
  (if _success
    (if (`self.GetCurve` "/Game/Systems/WaveSystem/AI_system/AI/BP_AI.BP_AI_C" "/Game/Systems/WaveSystem/Waves/CT_Waves.CT_Waves" (`self.GSCAbilitySystem`))
      (`AIBlueprintHelperLibrary.SpawnAIFromClass` (`self.GetRandomAi` (`self.GSCAbilitySystem`)) null _returnvalue (struct) false null)
      (return true))
    (else
      (return false))))

(fn `SpawnCharacter`
  (params (self2 :type "PC_TopDownShooter Object Reference"))
  (locals (Pawn :type "/Game/GameCore/Character/Characters/BP_CustomHUD_Character Class Reference" :default "/Script/Engine.BlueprintGeneratedClass'/Game/GameCore/Character/Characters/Warzog/BP_Warzog.BP_Warzog_C'") (PawnsList :type "Array of /Game/GameCore/Character/Characters/BP_CustomHUD_Character Class Reference"))
  (bind _returnvalue (`GameplayStatics.LoadGameFromSlot` "HERO"))
  (bind _assg_new_save_game (cast `/Game/Data/SaveGame/SG_NewSaveGame` _returnvalue)
    (:`then`
      (bind _hero (`/Game/Data/SaveGame/SG_NewSaveGame.HERO` _assg_new_save_game))
      (if (`KismetArrayLibrary.Array_Contains` (`local.PawnsList`) _hero)
        (set `local.Pawn` _hero)))
    (:`CastFailed`
      _))
  (`PC_TopDownShooter.spawnCharacter` self2 "/Game/GameCore/Character/Characters/Evilios/BP_Evilios.BP_Evilios_C"))

(fn `UserConstructionScript`)

(fn `WaveSystem`
  (bind _currentwave (`self.CurrentWave`))
  (bind _output (`|GetArrayItem` (`self.Waves`) _currentwave))
  (`/Engine/EditorBlueprintResources/StandardMacros.IsValid` _output :!label _label
    (:`Is Valid`
      (`self.startNewWave` _output)
      (set `self.CurrentWave` (+ _currentwave 1)))
    (:`Is Not Valid`
      (set `self.CurrentWave` 0)
      (goto _label))))