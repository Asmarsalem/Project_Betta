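; BP_HealthPotion is a loot pickup actor that applies a health potion effect to the player on overlap.
; When the overlapping actor is player character 0, it applies the GE_HealthPotion Gameplay Effect through that character's Ability System Component, then destroys itself.
; Both branches print the result of the player check as a debug string, and the construction script is empty.
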(event `self.ReceiveActorBeginOverlap`
  (params (OtherActor :type "Actor Object Reference"))
  (bind _returnvalue (`GameplayStatics.GetPlayerCharacter` 0))
  (bind _returnvalue_2 (== OtherActor _returnvalue))
  (if _returnvalue_2
    (`KismetSystemLibrary.PrintString` (`KismetStringLibrary.Conv_BoolToString` _returnvalue_2))
    (`AbilitySystemComponent.BP_ApplyGameplayEffectToSelf` (`AbilitySystemBlueprintLibrary.GetAbilitySystemComponent` _returnvalue) "/Game/GAS/GameplayEffects/GE_HealthPotion.GE_HealthPotion_C" 0.0 (make `GameplayEffectContextHandle`))
    (`self.K2_DestroyActor`)
    (else
      (`KismetSystemLibrary.PrintString` (`KismetStringLibrary.Conv_BoolToString` _returnvalue_2)))))

(fn `UserConstructionScript`)