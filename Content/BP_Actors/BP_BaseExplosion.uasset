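; BP_BaseExplosion is a base explosion actor that applies a Gameplay Effect to actors within its radius when it begins play.
; BeginPlay requires the player pawn to be BP_CustomHUD_Character, then spawns the damage emitter and sphere-traces one object type at its location.
; The player's Ability System Component applies EffectToActivate to each hit actor's component, making the player the effect's source.
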(event `self.ReceiveBeginPlay`
  (bind _returnvalue (`self.K2_GetActorLocation`))
  (bind _asbp_custom_hud_character (cast `/Game/Demo/Examples/CustomHUD/BP_CustomHUD_Character` (`GameplayStatics.GetPlayerCharacter` 0)))
  (`self.VFX`)
  (bind _outhits (`KismetSystemLibrary.SphereTraceMultiForObjects` _returnvalue _returnvalue (`self.Radius`) (`|MakeArray` "ObjectTypeQuery9" :!type "EObjectTypeQuery Enum")))
  (for _array_element _outhits
    (`AbilitySystemComponent.BP_ApplyGameplayEffectToTarget` :`self` (`AbilitySystemBlueprintLibrary.GetAbilitySystemComponent` _asbp_custom_hud_character) :`GameplayEffectClass` (`self.Effect To Activate`) :`Target` (`AbilitySystemBlueprintLibrary.GetAbilitySystemComponent` (`.HitActor` (`GameplayStatics.BreakHitResult` _array_element))))))

(event `VFX`
  (`GameplayStatics.SpawnEmitterAtLocation` (`self.Damage VFX`) (`self.K2_GetActorLocation`)))

(fn `UserConstructionScript`)