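; BP_AIBullet is a bullet actor, apparently fired by AI, that damages players through the Gameplay Ability System.
; On overlap it applies GE_ApplyDamage to actors that have an ability system component and implement BPI_Player.
; The effect's source is the ability system of an actor found with GetActorOfClass, rather than a stored shooter reference.
; Any overlap, player or not, also destroys the bullet after a short delay.
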(event `self.ReceiveActorBeginOverlap`
  (params (OtherActor :type "Actor Object Reference"))
  (bind _returnvalue (`AbilitySystemBlueprintLibrary.GetAbilitySystemComponent` OtherActor))
  (bind _returnvalue_2 (`GameplayStatics.GetActorOfClass` null))
  (`|ExecutionSequence`
    (:`then_0`
      (`KismetSystemLibrary.Delay` 0.3)
      (`self.K2_DestroyActor`))
    (:`then_1`
      (if (and (`KismetSystemLibrary.IsValid` _returnvalue) (`KismetSystemLibrary.DoesImplementInterface` OtherActor "/Game/Data/BP_Interface/BPI_Player.BPI_Player_C"))
        (`AbilitySystemComponent.BP_ApplyGameplayEffectToTarget` :`self` (`AbilitySystemBlueprintLibrary.GetAbilitySystemComponent` _returnvalue_2) :`GameplayEffectClass` "/Game/GAS/GameplayEffects/CharacterEffects/GE_ApplyDamage.GE_ApplyDamage_C" :`Target` _returnvalue)))))

(fn `UserConstructionScript`)