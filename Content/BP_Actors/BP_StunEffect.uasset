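; BP_StunEffect is an overlap-triggered actor that stuns enemies through the Gameplay Ability System.
; On overlap, it applies GE_Stun to the other actor if that actor has the Enemy tag and an ability system component, then prints an attribute value.
; Any overlap, enemy or not, also starts a short delay before the actor destroys itself.
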(event `self.ReceiveActorBeginOverlap`
  (params (OtherActor :type "Actor Object Reference"))
  (bind _returnvalue (`AbilitySystemBlueprintLibrary.GetAbilitySystemComponent` OtherActor))
  (`|ExecutionSequence`
    (:`then_0`
      (`KismetSystemLibrary.Delay` 0.4)
      (`self.K2_DestroyActor`))
    (:`then_1`
      (if (and (`self.ActorHasTag` OtherActor "Enemy") (`KismetSystemLibrary.IsValid` _returnvalue))
        (`AbilitySystemComponent.BP_ApplyGameplayEffectToSelf` :`self` _returnvalue :`GameplayEffectClass` "/Game/GAS/GameplayEffects/CharacterEffects/GE_Stun.GE_Stun_C")
        (`KismetSystemLibrary.PrintString` (`KismetStringLibrary.Conv_DoubleToString` (`.ReturnValue` (`AbilitySystemBlueprintLibrary.GetFloatAttributeFromAbilitySystemComponent` _returnvalue (struct :`AttributeName` "Speed" :`Attribute` "/Script/GASCompanionDemo.MainAttributes:Speed" :`AttributeOwner` "/Script/CoreUObject.Class'\"/Script/GASCompanionDemo.MainAttributes\"'")))))))))

(fn `UserConstructionScript`)