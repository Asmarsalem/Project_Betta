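; BP_HealthBooster is a reusable pickup actor that applies a health boost effect to players who overlap its sphere.
; On overlap, it checks that the other actor has an Ability System Component and implements BPI_Player, then applies GE_HealthBooster to that component.
; A CanBoostHealth flag and a Delay form a cooldown, so the booster re-arms itself after each use rather than being destroyed.
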(event `self.Sphere.OnComponentBeginOverlap`
  (params (OverlappedComponent :type "PrimitiveComponent Object Reference") (OtherActor :type "Actor Object Reference") (OtherComp :type "PrimitiveComponent Object Reference") (OtherBodyIndex :type Integer) (bFromSweep :type Boolean) (SweepResult :type "HitResult Structure (by ref)"))
  (bind _returnvalue (`AbilitySystemBlueprintLibrary.GetAbilitySystemComponent` OtherActor))
  (if (`self.CanBoostHealth`)
    (if (and (`KismetSystemLibrary.IsValid` _returnvalue) (`KismetSystemLibrary.DoesImplementInterface` OtherActor "/Game/Data/BP_Interface/BPI_Player.BPI_Player_C"))
      (`AbilitySystemComponent.BP_ApplyGameplayEffectToSelf` :`self` _returnvalue :`GameplayEffectClass` "/Game/GAS/GameplayEffects/GE_HealthBooster.GE_HealthBooster_C")
      (set `self.CanBoostHealth` false)
      (`KismetSystemLibrary.Delay` 15.0)
      (set `self.CanBoostHealth` true))))

(fn `UserConstructionScript`)