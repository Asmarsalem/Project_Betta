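; BP_BossBaseAbility is a base boss ability actor that applies a Gameplay Ability System effect to a player in its area when spawned.
; On BeginPlay it spawns an emitter through the VFX event, then runs a single-hit, zero-length sphere trace on the Camera channel, with debug drawing enabled.
; If the hit actor implements BPI_Player, EffectToApply is applied through that actor's ability system component.
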(event `self.ReceiveBeginPlay`
  (bind _returnvalue (`self.K2_GetActorLocation`))
  (`self.VFX`)
  (bind _outhit (`KismetSystemLibrary.SphereTraceSingle` :`Start` _returnvalue :`End` _returnvalue :`Radius` (`self.Radius`) :`TraceChannel` "TraceTypeQuery2" :`DrawDebugType` "ForDuration"))
  (bind (_bblockinghit _binitialoverlap _time _distance _location _impactpoint _normal _impactnormal _physmat _hitactor) (`GameplayStatics.BreakHitResult` _outhit))
  (if (`KismetSystemLibrary.DoesImplementInterface` _hitactor "/Game/Data/BP_Interface/BPI_Player.BPI_Player_C")
    (`AbilitySystemComponent.BP_ApplyGameplayEffectToSelf` :`self` (`AbilitySystemBlueprintLibrary.GetAbilitySystemComponent` _hitactor) :`GameplayEffectClass` (`self.Effect to apply`))))

(event `VFX`
  (`GameplayStatics.SpawnEmitterAtLocation` (`self.VEffect`) (`self.K2_GetActorLocation`)))

(fn `UserConstructionScript`)