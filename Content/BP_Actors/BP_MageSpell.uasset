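; BP_MageSpell is a projectile spell actor that applies a Gameplay Ability System effect to actors its box overlaps.
; On overlap, SpellDamage applies GameplayEffectClass to targets with a valid ability system component, using player 0's BP_CustomHUD_Character as source.
; SetParticleSpeed configures the projectile movement's speed and gravity scale.
; The delayed DestroyActor chain is unconnected, so this graph never destroys the spell.
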(event `self.ReceiveBeginPlay`)

(event `self.Box.OnComponentBeginOverlap`
  (params (OverlappedComponent :type "PrimitiveComponent Object Reference") (OtherActor :type "Actor Object Reference") (OtherComp :type "PrimitiveComponent Object Reference") (OtherBodyIndex :type Integer) (bFromSweep :type Boolean) (SweepResult :type "HitResult Structure (by ref)"))
  (bind _returnvalue (`AbilitySystemBlueprintLibrary.GetAbilitySystemComponent` OtherActor))
  (`self.SpellDamage` (`KismetSystemLibrary.IsValid` _returnvalue) _returnvalue))

(fn `Set particle speed`
  (params (InitialSpeed :type "Float (double-precision)") (MaxSpeed :type "Float (double-precision)") (Gravity :type "Float (double-precision)"))
  (bind _projectilemovement (`self.ProjectileMovement`))
  (set `ProjectileMovementComponent.InitialSpeed` InitialSpeed _projectilemovement)
  (set `ProjectileMovementComponent.MaxSpeed` MaxSpeed _projectilemovement)
  (set `ProjectileMovementComponent.ProjectileGravityScale` Gravity _projectilemovement))

(fn `SpellDamage`
  (params (`AbilitysystemValid?` :type Boolean) (EnemyAbilityComponent :type "AbilitySystemComponent Object Reference"))
  (bind _asbp_custom_hud_character (cast `/Game/GameCore/Character/Characters/BP_CustomHUD_Character` (`GameplayStatics.GetPlayerCharacter` 0)))
  (if `AbilitysystemValid?`
    (`AbilitySystemComponent.BP_ApplyGameplayEffectToTarget` :`self` (`AbilitySystemBlueprintLibrary.GetAbilitySystemComponent` _asbp_custom_hud_character) :`GameplayEffectClass` (`self.Gameplay Effect Class`) :`Target` EnemyAbilityComponent)))

(fn `UserConstructionScript`)